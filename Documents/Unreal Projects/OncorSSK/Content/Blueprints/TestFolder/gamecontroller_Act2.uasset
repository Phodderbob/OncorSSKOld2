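; Act 2 game controller that restores or initializes game state and spawns the player when the level begins.
; With a save present, it sends the saved GS value as a message, clearing the game instance's continued-from-previous-level flag and briefly delaying if that flag is set.
; Without one, it creates a save, stores GS_4 as the starting state and sends it.
; The player controller then spawns at a hardcoded location.
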(event EventBeginPlay
  (bind _savestruct (CallFunction|GetSave))
  (bind _gs (Utilities|Struct|BreakSave_Struct _savestruct))
  (if (.FoundSave (CallFunction|GetSave))
    (bind _asoncor_sskgame_instance (Utilities|Casting|CastToOncorSSKGame_Instance (Game|GetGameInstance)))
    (if (Variables|/Game/Blueprints/OncorSSKGame_Instance.OncorSSKGame_Instance_C|GetContinuedFromPreviousLevel _asoncor_sskgame_instance)
      (Variables|/Game/Blueprints/OncorSSKGame_Instance.OncorSSKGame_Instance_C|SetContinuedFromPreviousLevel _asoncor_sskgame_instance false)
      (CallFunction|Message _gs)
      (Utilities|FlowControl|Delay 0.2)
      (else
        (CallFunction|Message _gs :!label _label)))
    (else
      (CallFunction|NewSave)
      (Utilities|FlowControl|Delay 0.2)
      (CallFunction|SaveGameState "GS_4")
      (goto _label)))
  (bind _assskplayer_controller (Utilities|Casting|CastToSSKPlayerController (Game|GetPlayerController 0)))
  (Default|Spawn _assskplayer_controller "-221.000000,-6113.000000,-28.000000"))

(event EventTick
  (params (DeltaSeconds :type Float%20%28single-precision%29)))

(fn ConstructionScript
  (|CallParentFunction))