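; Act 3 game controller that sets up the level on BeginPlay by loading save state and spawning the player.
; Without a save, it creates one with game state GS_7; a flag on the game instance marks arrival from the previous level, clearing quests before spawn.
; All successful paths spawn through the SSK player controller, then pass the saved GS value to Message, with short delays sequencing the steps.
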(event EventBeginPlay
  (bind (_savestruct _foundsave) (CallFunction|GetSave))
  (Utilities|FlowControl|Delay 0.2)
  (if _foundsave
    (bind _asoncor_sskgame_instance (Utilities|Casting|CastToOncorSSKGame_Instance (Game|GetGameInstance))
      (:then
        (if (Variables|/Game/Blueprints/OncorSSKGame_Instance.OncorSSKGame_Instance_C|GetContinuedFromPreviousLevel _asoncor_sskgame_instance)
          (Variables|/Game/Blueprints/OncorSSKGame_Instance.OncorSSKGame_Instance_C|SetContinuedFromPreviousLevel _asoncor_sskgame_instance false)
          (Utilities|FlowControl|Delay 0.2)
          (CallFunction|ClearQuests)
          (bind _assskplayer_controller (Utilities|Casting|CastToSSKPlayerController (Game|GetPlayerController 0)))
          (Default|Spawn _assskplayer_controller "0, 0, 0")
          (CallFunction|Message (.GS (Utilities|Struct|BreakSave_Struct _savestruct)) :!label _label)
          (else
            (bind _assskplayer_controller_2 (Utilities|Casting|CastToSSKPlayerController (Game|GetPlayerController 0) :!label _label_2)
              (:then
                (Utilities|FlowControl|Delay 0.2)
                (Default|Spawn _assskplayer_controller_2 "0, 0, 0")
                (goto _label))
              (:CastFailed
                (Development|PrintString "SSKControllerNotFound"))))))
      (:CastFailed
        (Development|PrintString "GameInstanceCastFaile")))
    (else
      (CallFunction|NewSave)
      (Utilities|FlowControl|Delay 0.2)
      (CallFunction|SaveGameState "GS_7")
      (Utilities|FlowControl|Delay 0.2)
      (goto _label_2))))

(fn ConstructionScript
  (|CallParentFunction))