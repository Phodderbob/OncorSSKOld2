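; Game-progression controller that reacts to game-state strings sent through Message in the Oncor neighborhood levels.
; Specific state and level pairs open the next act behind a loading screen, saving state and clearing quests, or wipe the save and restart after Act 3.
; Other states use GameStates table rows to toggle streaming-level visibility, hide saved completed levels, then refresh POI icons.
; Some states also swap the player's music after a delay.
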(event Custom|Update%20Triggers
  (bind _outactors (Actor|GetAllActorsOfClass "/Game/Blueprints/Trigger.Trigger_C"))
  (for _array_element _outactors
    (Utilities|IsValid (Variables|/Game/Blueprints/Trigger.Trigger_C|GetPOI_Component _array_element)
      (:Is%20Valid
        (Default|UpdateIcon (Variables|/Game/Blueprints/Trigger.Trigger_C|GetPOI_Component _array_element)))))
  (bind _outactors_2 (Actor|GetAllActorsOfClass "/Game/Blueprints/HiddenObjectController.HiddenObjectController_C"))
  (for _array_element_2 _outactors_2
    (Default|UpdateIcon (Variables|/Game/Blueprints/HiddenObjectController.HiddenObjectController_C|GetPOI_Component _array_element_2))))

(event Custom|UpdateIcons
  ;[1 1 1] Update Icons
  (bind _outactors (Actor|GetAllActorsOfClass "/Game/Blueprints/Trigger.Trigger_C"))
  (for _array_element _outactors
    (Utilities|IsValid (Variables|/Game/Blueprints/Trigger.Trigger_C|GetPOI_Component _array_element)
      (:Is%20Valid
        (Default|UpdateIcon (Variables|/Game/Blueprints/Trigger.Trigger_C|GetPOI_Component _array_element))))))

(event EventBeginPlay)

(event EventMessage
  (params (String :type String))
  (bind _output_get (Variables|Default|SetCurrentState String))
  (Utilities|FlowControl|Sequence
    (:then_0
      (bind _returnvalue (Game|GetCurrentLevelName true))
      (if (and (Utilities|Enum|Equal(Enum) _output_get "GS_4") (Utilities|Enum|Equal(Enum) _returnvalue "OncorNeighorhood"))
        ;[1 1 1] Transition to Act 2
        (bind _returnvalue_2 (UserInterface|CreateWidget "/Game/Blueprints/Widget/LoadingScreen.LoadingScreen_C"))
        (UserInterface|Viewport|AddtoViewport _returnvalue_2 0)
        (CallFunction|ClearQuests)
        (Utilities|FlowControl|Delay 0.2)
        (CallFunction|SaveGameState "GS_4")
        (bind _asoncor_sskgame_instance (Utilities|Casting|CastToOncorSSKGame_Instance (Game|GetGameInstance)))
        (Variables|/Game/Blueprints/OncorSSKGame_Instance.OncorSSKGame_Instance_C|SetContinuedFromPreviousLevel _asoncor_sskgame_instance true)
        (Utilities|FlowControl|Delay 0.2)
        (CallFunction|ClearQuests)
        (Utilities|FlowControl|Delay 0.2)
        (Game|OpenLevel(byName) "OncorNeighorhoodACT2")
        (elif (and (Utilities|Enum|Equal(Enum) _returnvalue "OncorNeighorhoodACT2") (Utilities|Enum|Equal(Enum) _output_get "GS_7"))
          ;[1 1 1] Transition to Act 3
          (bind _returnvalue_3 (UserInterface|CreateWidget "/Game/Blueprints/Widget/LoadingScreen.LoadingScreen_C"))
          (UserInterface|Viewport|AddtoViewport _returnvalue_3 0)
          (CallFunction|ClearQuests)
          (Utilities|FlowControl|Delay 0.2)
          (CallFunction|SaveGameState "GS_7")
          (Utilities|FlowControl|Delay 0.2)
          (CallFunction|ClearQuests)
          (bind _asoncor_sskgame_instance_2 (Utilities|Casting|CastToOncorSSKGame_Instance (Game|GetGameInstance)))
          (Variables|/Game/Blueprints/OncorSSKGame_Instance.OncorSSKGame_Instance_C|SetContinuedFromPreviousLevel _asoncor_sskgame_instance_2 true)
          (Utilities|FlowControl|Delay 0.2)
          (Game|OpenLevel(byName) "OncorNeighorhoodAct3")
          (elif (and (Utilities|Enum|Equal(Enum) _returnvalue "OncorNeighorhoodAct3") (Utilities|Enum|Equal(Enum) _output_get "GS_10"))
            (CallFunction|ClearSave)
            (Game|OpenLevel(byName) "OncorNeighorhood")
            (else
              (bind _returnvalue_4 (Utilities|GetDataTableRow (Variables|Default|GetGame_States) (Utilities|String|StringToName String))
                (:then
                  (Variables|Default|SetLevels (Utilities|String|ParseIntoArray (.LevelstoLoad (Utilities|Struct|Breakgame_State _returnvalue_4)) ","))
                  (Variables|Default|SetUnLevels (Utilities|String|ParseIntoArray (.LevelstoUnload (Utilities|Struct|Breakgame_State _returnvalue_4)) ","))
                  ;[1 1 1] show Levels
                  (for _array_element (Variables|Default|GetLevels)
                    (Utilities|IsValid (Class|GameplayStatics|GetStreamingLevel (Utilities|String|StringToName _array_element))
                      (:Is%20Valid
                        (Variables|/Script/Engine.LevelStreaming|SetbShouldBeVisible (Class|GameplayStatics|GetStreamingLevel (Utilities|String|StringToName _array_element)) true))))
                  ;[1 1 1] Hide Levels
                  (for _array_element_2 (Variables|Default|GetUnLevels)
                    (Utilities|IsValid (Class|GameplayStatics|GetStreamingLevel (Utilities|String|StringToName _array_element_2))
                      (:Is%20Valid
                        (Variables|/Script/Engine.LevelStreaming|SetbShouldBeVisible (Class|GameplayStatics|GetStreamingLevel (Utilities|String|StringToName _array_element_2)) false))))
                  ;[0.01492 1 0] Hide all Trigger boxes that have been prevously saved.
                  (for _array_element_3 (.Completed_Lvls (Utilities|Struct|BreakSave_Struct (.SaveStruct (CallFunction|GetSave))))
                    (Utilities|IsValid (Class|GameplayStatics|GetStreamingLevel (Utilities|String|StringToName _array_element_3))
                      (:Is%20Valid
                        (Variables|/Script/Engine.LevelStreaming|SetbShouldBeVisible (Class|GameplayStatics|GetStreamingLevel (Utilities|String|StringToName _array_element_3)) false))))
                  (Utilities|FlowControl|Sequence
                    (:then_1
                      (Utilities|FlowControl|Delay 1.0)
                      (Default|CallCallPlayonSpawn)
                      (Default|CallStaticInitialize)
                      (CallFunction|UpdateIcons))))
                (:RowNotFound
                  (Development|PrintString "GS Row Not Found"))))))))
    (:then_1
      (Utilities|FlowControl|Delay 1.0)
      (if (Utilities|Enum|Equal(Enum) _output_get "GS_3")
        (bind _asthird_person_character (Utilities|Casting|CastToThirdPersonCharacter (Game|Player|GetPlayerPawn 0)))
        (Audio|Components|Audio|SetSound (Variables|/Game/ThirdPersonBP/Blueprints/ThirdPersonCharacter.ThirdPersonCharacter_C|GetMusic _asthird_person_character) "/Game/Audio/Music/Tenth_Nail.Tenth_Nail")
        (elif (Utilities|Enum|Equal(Enum) _output_get "GS_4")
          (bind _asthird_person_character_2 (Utilities|Casting|CastToThirdPersonCharacter (Game|Player|GetPlayerPawn 0)))
          (Audio|Components|Audio|SetSound (Variables|/Game/ThirdPersonBP/Blueprints/ThirdPersonCharacter.ThirdPersonCharacter_C|GetMusic _asthird_person_character_2) "/Game/Audio/Music/249_loop2_lazy-afternoon_0012_Cue.249_loop2_lazy-afternoon_0012_Cue")
          (elif (Utilities|Enum|Equal(Enum) _output_get "GS_6")
            (bind _asthird_person_character_3 (Utilities|Casting|CastToThirdPersonCharacter (Game|Player|GetPlayerPawn 0)))
            (Audio|Components|Audio|SetSound (Variables|/Game/ThirdPersonBP/Blueprints/ThirdPersonCharacter.ThirdPersonCharacter_C|GetMusic _asthird_person_character_3) "/Game/Audio/Music/249_loop2_lazy-afternoon_0012_Cue.249_loop2_lazy-afternoon_0012_Cue")
            (elif (Utilities|Enum|Equal(Enum) _output_get "GS_6")
              (bind _asthird_person_character_4 (Utilities|Casting|CastToThirdPersonCharacter (Game|Player|GetPlayerPawn 0)))
              (Audio|Components|Audio|SetSound (Variables|/Game/ThirdPersonBP/Blueprints/ThirdPersonCharacter.ThirdPersonCharacter_C|GetMusic _asthird_person_character_4) "/Game/Audio/Music/249_loop6_lazy-afternoon_0027_Cue.249_loop6_lazy-afternoon_0027_Cue"))))))))

(event EventUnhideLevelUpdatePOI
  (params (LevelName :type String))
  (Variables|/Script/Engine.LevelStreaming|SetbShouldBeVisible (Class|GameplayStatics|GetStreamingLevel (Utilities|String|StringToName LevelName)) true))

(fn ConstructionScript)

(fn LevelsinGameState
  (params (GS :type String))
  (bind _returnvalue (Utilities|GetDataTableRow (Variables|Default|GetGame_States) (Utilities|String|StringToName GS))
    (:then
      (return (Utilities|String|ParseIntoArray (.LevelstoLoad (Utilities|Struct|Breakgame_State _returnvalue)) ",")))))