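; Blueprint function library that manages the game's single "Save" slot, covering player profile, game state, quests, completed levels and volumes.
; Save and GetSave wrap SSK_Save_Game slot I/O; helpers read the struct, change one field and rewrite it whole.
; AddQuest, RemoveQuest and AddCompletedLevel omit volume fields when rebuilding.
; ClearQuests also resets volumes and empties the HUD quest box, while other functions seed, delete or print the save.
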(fn Save
  (params (SaveStruct :type Save%20Struct%20Structure))
  (bind _returnvalue (SaveGame|CreateSaveGameObject "/Game/Blueprints/SSK_Save_Game.SSK_Save_Game_C"))
  (bind _asssk_save_game (Utilities|Casting|CastToSSK_Save_Game _returnvalue))
  (Variables|/Game/Blueprints/SSK_Save_Game.SSK_Save_Game_C|SetSave _asssk_save_game SaveStruct)
  (bind _returnvalue_2 (SaveGame|SaveGametoSlot _returnvalue "Save"))
  (return _returnvalue_2))

(fn GetSave
  (bind _returnvalue (SaveGame|DoesSaveGameExist "Save"))
  (bind _returnvalue_2 (SaveGame|LoadGamefromSlot "Save"))
  (bind _asssk_save_game (Utilities|Casting|CastToSSK_Save_Game _returnvalue_2)
    (:then
      (if _returnvalue
        (return (Variables|/Game/Blueprints/SSK_Save_Game.SSK_Save_Game_C|GetSave _asssk_save_game) true)
        (else
          _)))
    (:CastFailed
      _))
  (return "" false))

(fn ClearSave
  (bind _returnvalue (SaveGame|DeleteGameinSlot "Save"))
  (return _returnvalue))

(fn ClearQuests
  (bind _returnvalue (SaveGame|DoesSaveGameExist "Save"))
  (if _returnvalue
    (bind _returnvalue_2 (SaveGame|LoadGamefromSlot "Save"))
    (bind _asssk_save_game (Utilities|Casting|CastToSSK_Save_Game _returnvalue_2)
      (:then
        (bind _returnvalue_3 (SaveGame|CreateSaveGameObject "/Game/Blueprints/SSK_Save_Game.SSK_Save_Game_C"))
        (bind _output_get (Variables|/Game/Blueprints/SSK_Save_Game.SSK_Save_Game_C|SetSave _returnvalue_3 (Utilities|Struct|MakeSave_Struct (.gs (Variables|/Game/Blueprints/SSK_Save_Game.SSK_Save_Game_C|GetSave _asssk_save_game)) (.collectables (Variables|/Game/Blueprints/SSK_Save_Game.SSK_Save_Game_C|GetSave _asssk_save_game)) (.gender (Variables|/Game/Blueprints/SSK_Save_Game.SSK_Save_Game_C|GetSave _asssk_save_game)) (.ethnicity (Variables|/Game/Blueprints/SSK_Save_Game.SSK_Save_Game_C|GetSave _asssk_save_game)) (.languages (Variables|/Game/Blueprints/SSK_Save_Game.SSK_Save_Game_C|GetSave _asssk_save_game)) (.player_location (Variables|/Game/Blueprints/SSK_Save_Game.SSK_Save_Game_C|GetSave _asssk_save_game)) (.tutorialcompleted? (Variables|/Game/Blueprints/SSK_Save_Game.SSK_Save_Game_C|GetSave _asssk_save_game)) (.completed_minigames (Variables|/Game/Blueprints/SSK_Save_Game.SSK_Save_Game_C|GetSave _asssk_save_game)) (.completed_lvls (Variables|/Game/Blueprints/SSK_Save_Game.SSK_Save_Game_C|GetSave _asssk_save_game)) (Utilities|Array|MakeArray (Utilities|Struct|MakeQuestSaveStruct "NewEnumerator6" 0 0)) 0.5 0.5)))
        (bind _asthird_person_character (Utilities|Casting|CastToThirdPersonCharacter (Game|Player|GetPlayerPawn 0)))
        (Widget|Panel|ClearChildren (Variables|/Game/Blueprints/SSK_HUD.SSK_HUD_C|GetQuestBox (Variables|/Game/ThirdPersonBP/Blueprints/ThirdPersonCharacter.ThirdPersonCharacter_C|GetHud _asthird_person_character)))
        (bind _success (CallFunction|Save _output_get (LocalVariables|Get__WorldContext)))
        (if _success
          (return true)
          (else
            _)))
      (:CastFailed
        _)))
  (return false))

(fn AddQuest
  (params (QuestSaveStruct :type Quest%20Save%20Struct%20Structure))
  (bind ___worldcontext (LocalVariables|Get__WorldContext))
  (bind (_savestruct _foundsave) (CallFunction|GetSave ___worldcontext))
  (bind (_gs _collectables _gender _ethnicity _languages _player_location _tutorialcompleted_ _completed_minigames _completed_lvls _currentquests) (Utilities|Struct|BreakSave_Struct _savestruct))
  (if _foundsave
    (bind _output_get (LocalVariables|SetCurrentQuests _currentquests))
    (Utilities|Array|AddUnique _output_get QuestSaveStruct)
    (bind _success (CallFunction|Save (Utilities|Struct|MakeSave_Struct _gs _collectables _gender _ethnicity _languages _player_location _tutorialcompleted_ _completed_minigames _completed_lvls _output_get 0.5 0.5) (LocalVariables|Get__WorldContext)))
    (if _success
      (return true)
      (else
        _)))
  (return false))

(fn SaveQuest
  (params (QuestSaveStruct :type Quest%20Save%20Struct%20Structure))
  (bind (_quest _currentobject _currentvalue) (Utilities|Struct|BreakQuestSaveStruct QuestSaveStruct))
  (bind ___worldcontext (LocalVariables|Get__WorldContext))
  (bind (_savestruct _foundsave) (CallFunction|GetSave ___worldcontext))
  (bind (_gs _collectables _gender _ethnicity _languages _player_location _tutorialcompleted_ _completed_minigames _completed_lvls _currentquests _musicvolume _sfxvolume) (Utilities|Struct|BreakSave_Struct _savestruct))
  (if _foundsave
    (bind _output_get (LocalVariables|SetQuests _currentquests))
    (for (_array_element _array_index) _output_get
      (if (Utilities|Enum|Equal(Enum) (.Quest (Utilities|Struct|BreakQuestSaveStruct _array_element)) _quest)
        (Utilities|Array|SetArrayElem _output_get _array_index (Utilities|Struct|MakeQuestSaveStruct (.Quest (Utilities|Struct|BreakQuestSaveStruct _array_element)) _currentobject _currentvalue))
        (bind _success (CallFunction|Save (Utilities|Struct|MakeSave_Struct _gs _collectables _gender _ethnicity _languages _player_location _tutorialcompleted_ _completed_minigames _completed_lvls (LocalVariables|GetQuests) _musicvolume _sfxvolume) (LocalVariables|Get__WorldContext)))
        (return _success)))
    (else
      (return false))))

(fn RemoveQuest
  (params (QuestSave :type ClickableObjectType%20Enum :default "NewEnumerator0"))
  (bind ___worldcontext (LocalVariables|Get__WorldContext))
  (bind (_savestruct _foundsave) (CallFunction|GetSave ___worldcontext))
  (bind (_gs _collectables _gender _ethnicity _languages _player_location _tutorialcompleted_ _completed_minigames _completed_lvls _currentquests) (Utilities|Struct|BreakSave_Struct _savestruct))
  (if _foundsave
    (bind _output_get (LocalVariables|SetQuests _currentquests))
    (for (_array_element _array_index) _output_get
      (if (Utilities|Enum|Equal(Enum) (.Quest (Utilities|Struct|BreakQuestSaveStruct _array_element)) QuestSave)
        (Utilities|Array|RemoveIndex (LocalVariables|GetQuests) _array_index)
        (bind _success (CallFunction|Save (Utilities|Struct|MakeSave_Struct _gs _collectables _gender _ethnicity _languages _player_location _tutorialcompleted_ _completed_minigames _completed_lvls (LocalVariables|GetQuests) 0.5 0.5) (LocalVariables|Get__WorldContext)))
        (return _success)))
    (else
      (return false))))

(fn SaveGameState
  (params (GS :type String))
  (bind ___worldcontext (LocalVariables|Get__WorldContext))
  (bind (_savestruct _foundsave) (CallFunction|GetSave ___worldcontext))
  (if _foundsave
    (bind _success (CallFunction|Save (Utilities|Struct|MakeSave_Struct GS (.collectables _savestruct) (.gender _savestruct) (.ethnicity _savestruct) (.languages _savestruct) (.player_location _savestruct) (.tutorialcompleted? _savestruct) (.completed_minigames _savestruct) (.completed_lvls _savestruct) (.currentquests _savestruct) (.musicvolume _savestruct) (.sfxvolume _savestruct)) ___worldcontext))
    (return _success)
    (else
      (return false))))

(fn AddCompletedLevel
  (params (Level :type String))
  (bind ___worldcontext (LocalVariables|Get__WorldContext))
  (bind (_savestruct _foundsave) (CallFunction|GetSave ___worldcontext))
  (bind (_gs _collectables _gender _ethnicity _languages _player_location _tutorialcompleted_ _completed_minigames _completed_lvls _currentquests) (Utilities|Struct|BreakSave_Struct _savestruct))
  (if _foundsave
    (bind _output_get (LocalVariables|SetCompleted _completed_lvls))
    (Utilities|Array|AddUnique _output_get Level)
    (bind _success (CallFunction|Save (Utilities|Struct|MakeSave_Struct _gs _collectables _gender _ethnicity _languages _player_location _tutorialcompleted_ _completed_minigames (LocalVariables|GetCompleted) _currentquests 0.5 0.5) (LocalVariables|Get__WorldContext)))
    (return _success)
    (else
      (return false))))

(fn NewSave
  (CallFunction|Save (Utilities|Struct|MakeSave_Struct "GS_1" (Utilities|Array|MakeArray "") true "NewEnumerator0" "NewEnumerator0" "0, 0, 0" false (Utilities|Array|MakeArray "0, 0, 0") (Utilities|Array|MakeArray "") (Utilities|Array|MakeArray (Utilities|Struct|MakeQuestSaveStruct "NewEnumerator6")) 0.5 0.5) (LocalVariables|Get__WorldContext)))

(fn PrintSaveData
  (bind ___worldcontext (LocalVariables|Get__WorldContext))
  (bind ___worldcontext_2 (LocalVariables|Get__WorldContext))
  (bind (_savestruct _foundsave) (CallFunction|GetSave ___worldcontext))
  (bind (_gs _collectables _gender _ethnicity _languages _player_location _tutorialcompleted_ _completed_minigames _completed_lvls _currentquests _musicvolume _sfxvolume) (Utilities|Struct|BreakSave_Struct _savestruct))
  (if _foundsave
    (Development|PrintString ___worldcontext_2 (Utilities|String|Append "GameState: " _gs))
    (Development|PrintString ___worldcontext_2 (Utilities|String|Append "Gendermale; " (Utilities|String|ToString(Boolean) _gender)))
    (Development|PrintString ___worldcontext_2 (Utilities|String|Append "Ethnicity: " (Utilities|String|EnumtoString _ethnicity)))
    (Development|PrintString ___worldcontext_2 (Utilities|String|Append "Language: " (Utilities|String|EnumtoString _languages)))
    (Development|PrintString ___worldcontext_2 (Utilities|String|Append "TutorialComplete: " (Utilities|String|ToString(Boolean) _tutorialcompleted_)))
    (Development|PrintString ___worldcontext_2 "Completed Levels")
    (for _array_element _completed_lvls
      (Development|PrintString 0 _array_element))
    (Development|PrintString 0 "Current Quests")
    (for _array_element_2 _currentquests
      (Development|PrintString 0 (Utilities|String|EnumtoString (.quest _array_element_2))))
    (Development|PrintString 0 (Utilities|String|Append "Music Volume: " (Utilities|String|ToString(Float) _musicvolume)))
    (Development|PrintString 0 (Utilities|String|Append "SFX Volume: " (Utilities|String|ToString(Float) _sfxvolume)))
    (else
      (Development|PrintString ___worldcontext "NoSaveFound"))))