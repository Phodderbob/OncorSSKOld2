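; Player controller that spawns and possesses the player's character from the saved gender and ethnicity.
; It starts in UI-only input; the Spawn event uses a custom location, or a PlayerStart's location when that is zero.
; Male and female spawning macros pick the character class, then switch to game-only input.
; Input actions track keyboard versus controller use; the no-save fallback and on-spawn dialogue logic are unconnected.
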(event Custom|Spawn
  (params (CustomLocation :type Vector))
  (bind (_savestruct _foundsave) (CallFunction|GetSave))
  (bind (_gs _collectables _gender _ethnicity) (Utilities|Struct|BreakSave_Struct _savestruct))
  (if (Math|Vector|Equal(Vector) CustomLocation "0, 0, 0" 0.0001)
    (bind _outactors (Actor|GetAllActorsOfClass "/Script/Engine.PlayerStart"))
    (for _array_element _outactors
      (Variables|Default|SetSpawn%20Transform (Math|Transform|MakeTransform (Transformation|GetActorLocation _array_element) "0, 0, 0" "1,1,1")))
    (else
      (Variables|Default|SetSpawn%20Transform (Math|Transform|MakeTransform CustomLocation "0, 0, 0" "1,1,1"))))
  (if _foundsave
    ;[1 1 1] Boy=True Girl=False
    (if _gender
      (Development|PrintString (Utilities|String|EnumtoString _ethnicity) true true "(R=0.000000,G=1.000000,B=0.298514,A=1.000000)" 5.0)
      (switch Utilities|FlowControl|Switch|SwitchonEthnicity _ethnicity
        (:NewEnumerator0
          (|MaleModdleSpawning (Variables|Default|GetSpawn%20Transform) :!label _label))
        (:NewEnumerator1
          (goto _label Black))
        (:NewEnumerator2
          (goto _label Latino))
        (:NewEnumerator3
          (goto _label Asian)))
      (else
        (Development|PrintString (Utilities|String|EnumtoString _ethnicity) true true "(R=1.000000,G=0.000000,B=0.000000,A=1.000000)" 5.0)
        (switch Utilities|FlowControl|Switch|SwitchonEthnicity _ethnicity
          (:NewEnumerator0
            (|FemaleModdleSpawning (Variables|Default|GetSpawn%20Transform) :!label _label_2))
          (:NewEnumerator1
            (goto _label_2 Black))
          (:NewEnumerator2
            (goto _label_2 Latino))
          (:NewEnumerator3
            (goto _label_2 Asian)))))))

(event EventBeginPlay
  (Input|SetInputModeUIOnly self 0 "DoNotLock"))

(event Input|ActionEvents|InputActionControllerInput
  (params (Key :type Key%20Structure))
  (:Pressed
    (if (Game|Player|IsInputKeyDown (Game|GetPlayerController 0) Key)
      (Variables|Default|SetController? true)
      (Development|PrintString (Utilities|String|ToString(Boolean) (Variables|Default|GetController?))))))

(event Input|ActionEvents|InputActionKeyboardInput
  (params (Key :type Key%20Structure))
  (:Pressed
    (if (Game|Player|IsInputKeyDown (Game|GetPlayerController 0) Key)
      (Variables|Default|SetController? false)
      (Development|PrintString (Utilities|String|ToString(Boolean) (Variables|Default|GetController?))))))

(fn ConstructionScript)