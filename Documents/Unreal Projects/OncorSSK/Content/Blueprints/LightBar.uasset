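; LightBar is a Blueprint for a flashing light bar that alternates two groups of lights in an endless loop.
; Each group is a custom event that shows or hides its static meshes and activates or deactivates the matching point lights.
; BeginPlay switches one group on and the other off, waits half a second, swaps them, waits again and loops back.
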(event Custom|Group2
  (params (On? :type Boolean))
  (if On?
    ;[1 1 1] Group 2 On
    (for _array_element (Utilities|Array|MakeArray (Variables|Default|GetStaticMesh) (Variables|Default|GetStaticMesh2))
      (Development|SetHiddeninGame _array_element false false))
    (for _array_element_2 (Utilities|Array|MakeArray (Variables|Default|GetPointLight) (Variables|Default|GetPointLight2))
      (Components|Activation|SetActive _array_element_2 true false))
    (else
      ;[1 1 1] Group 2 Off
      (for _array_element_3 (Utilities|Array|MakeArray (Variables|Default|GetStaticMesh) (Variables|Default|GetStaticMesh2))
        (Development|SetHiddeninGame _array_element_3 true false))
      (for _array_element_4 (Utilities|Array|MakeArray (Variables|Default|GetPointLight) (Variables|Default|GetPointLight2))
        (Components|Activation|SetActive _array_element_4 false false)))))

(event Custom|Group1
  (params (On? :type Boolean))
  (if On?
    ;[1 1 1] Group 1 On
    (for _array_element (Utilities|Array|MakeArray (Variables|Debug|GetStaticMeshComponent) (Variables|Default|GetStaticMesh1) (Variables|Default|GetStaticMesh3))
      (Development|SetHiddeninGame _array_element false false))
    (for _array_element_2 (Utilities|Array|MakeArray (Variables|Default|GetPointLight3) (Variables|Default|GetPointLight1) (Variables|Default|GetPointLight4))
      (Components|Activation|SetActive _array_element_2 true false))
    (else
      ;[1 1 1] Group 1 Off
      (for _array_element_3 (Utilities|Array|MakeArray (Variables|Debug|GetStaticMeshComponent) (Variables|Default|GetStaticMesh1) (Variables|Default|GetStaticMesh3))
        (Development|SetHiddeninGame _array_element_3 true false))
      (for _array_element_4 (Utilities|Array|MakeArray (Variables|Default|GetPointLight3) (Variables|Default|GetPointLight1) (Variables|Default|GetPointLight4))
        (Components|Activation|SetActive _array_element_4 false false)))))

(event EventBeginPlay
  (CallFunction|Group1 true :!label _label)
  (CallFunction|Group2 false)
  (Utilities|FlowControl|Delay 0.5)
  (CallFunction|Group1 false)
  (CallFunction|Group2 true)
  (Utilities|FlowControl|Delay 0.5)
  (goto _label))

(event Collision|EventActorBeginOverlap
  (params (OtherActor :type Actor%20Object%20Reference)))

(fn ConstructionScript)