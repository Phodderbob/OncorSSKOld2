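; Clickable cat actor for what appears to be a hidden-object game.
; On BeginPlay it caches all CatTPoint actors, prints their count and binds CatClicked as its click handler.
; A click prints a debug message, calls CatObj on HiddenObjectController, runs two MoveComponentTo calls on its Cube and increments a counter.
; The cached points feed nothing, and neither move shows a target location.
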(event Custom|CatClicked
  (bind _cube (Variables|Default|GetCube))
  (Development|PrintString "Hello" true true "(R=0.068677,G=0.026278,B=1.000000,A=1.000000)")
  (Default|CatObj (Variables|Default|GetHiddenObjectController))
  (Components|MoveComponentTo _cube "0, 0, 0" "0, 0, 0" false false 2.0 false)
  (Components|MoveComponentTo _cube "0, 0, 0" "0, 0, 0" false false 0.0 false)
  (Math|Integer|IncrementInt (Variables|Default|GetNewVar_1)))

(event EventBeginPlay
  (|CallParentFunction)
  (bind _outactors (Actor|GetAllActorsOfClass "/Game/Blueprints/CatTPoint.CatTPoint_C"))
  (Variables|Default|SetCatTPoints _outactors)
  (EventDispatchers|BindEventtoClicked (delegate Custom|CatClicked))
  (Development|PrintString (Utilities|String|ToString(Integer) (Utilities|Array|Length (Variables|Default|GetCatTPoints))) true true "(R=1.000000,G=0.141020,B=0.341967,A=1.000000)"))

(event Collision|EventActorBeginOverlap
  (params (OtherActor :type Actor%20Object%20Reference))
  (|CallParentFunction OtherActor) ; This node is disabled and will not be called.\nDrag off pins to build functionality.
)

(event EventTick
  (params (DeltaSeconds :type Float%20%28single-precision%29))
  (|CallParentFunction DeltaSeconds) ; This node is disabled and will not be called.\nDrag off pins to build functionality.
)

(fn ConstructionScript
  (|CallParentFunction))