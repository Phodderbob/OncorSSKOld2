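; Out-of-bounds volume that gives the player a few seconds to leave before moving them back into play.
; Overlap shows a countdown widget driven by a looping timer; leaving clears the timer and resets the count.
; At zero, ReLocat moves the player to the first TargetPoint found, between fade-out and fade-in animations.
; Paired DoOnce gates re-arm enter and exit handling, while StillTP keeps the widget alive during relocation.
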(event OnComponentBeginOverlap(OutofBounceBox)
  (params (OverlappedComponent :type Primitive%20Component%20Object%20Reference) (OtherActor :type Actor%20Object%20Reference) (OtherComp :type Primitive%20Component%20Object%20Reference) (OtherBodyIndex :type Integer) (bFromSweep :type Boolean) (SweepResult :type Hit%20Result%20Structure%20%28by%20ref%29))
  ;[0 1 0.2985] When Player Over laps OOB Box, they have 5 second to get out.
  (Utilities|Casting|CastToThirdPersonCharacter OtherActor)
  (Utilities|FlowControl|DoOnce false
    (:Completed
      (Variables|Default|SetStill_OOB? true)
      (bind _returnvalue (UserInterface|CreateWidget "/Game/Blueprints/Widget/out_of_bounce_Widget.out_of_bounce_Widget_C" (Game|GetPlayerController 0)))
      (bind _output_get (Variables|Default|SetOOB_widget _returnvalue))
      (UserInterface|Viewport|AddtoViewport _output_get 0)
      (Utilities|FlowControl|Sequence
        (:then_0
          (CallFunction|RestartEnd))
        (:then_1
          (Utilities|FlowControl|Delay 1.0)
          (Utilities|Time|SetTimerbyFunctionName 0 "CountDown" 1.0 (Variables|Default|GetStill_OOB?)))))))

(event OnComponentEndOverlap(OutofBounceBox)
  (params (OverlappedComponent :type Primitive%20Component%20Object%20Reference) (OtherActor :type Actor%20Object%20Reference) (OtherComp :type Primitive%20Component%20Object%20Reference) (OtherBodyIndex :type Integer))
  ;[1 1 1] When Player end overlap, It will restart all vars .
  (Utilities|Casting|CastToThirdPersonCharacter OtherActor)
  (Utilities|Time|ClearTimerbyFunctionName 0 "CountDown")
  (Variables|Default|SetStill_OOB? false)
  (Variables|Default|SetTimer 6)
  (Variables|/Game/Blueprints/Widget/out_of_bounce_Widget.out_of_bounce_Widget_C|SetOOB_text (Variables|Default|GetOOB_widget) "")
  (Utilities|FlowControl|DoOnce true
    (:Completed
      (if (not (Variables|Default|GetStill%20TP?))
        (Widget|RemovefromParent (Variables|Default|GetOOB_widget))
        (CallFunction|RestartBegin)))))

(event Custom|CountDown
  ;[1 0 0] Count down to five second before calling Re Locat
  (bind _result (Math|Integer|DecrementInt (Variables|Default|GetTimer))
    (:%20%20
      (Variables|/Game/Blueprints/Widget/out_of_bounce_Widget.out_of_bounce_Widget_C|SetOOB_text (Variables|Default|GetOOB_widget) (Utilities|String|Append "You Have " (Utilities|String|ToString(Integer) _result) " Seconds!"))
      (if (== (Variables|Default|GetTimer) 0)
        (Variables|/Game/Blueprints/Widget/out_of_bounce_Widget.out_of_bounce_Widget_C|SetOOB_text (Variables|Default|GetOOB_widget) "")
        (CallFunction|ReLocat)))))

(event Custom|ReLocat
  (bind _oob_widget (Variables|Default|GetOOB_widget))
  (bind _oob_widget_2 (Variables|Default|GetOOB_widget))
  ;[1 0.8528 0.04501] TP player back to Target Point during Fade Out and Fade In.  Then remvoe widget from Parent.
  (Variables|Default|SetStill%20TP? true)
  (UserInterface|Animation|PlayAnimation _oob_widget (Variables|/Game/Blueprints/Widget/out_of_bounce_Widget.out_of_bounce_Widget_C|GetFadeOut _oob_widget) 0.0 1 "Forward" 1.0)
  (Utilities|FlowControl|Delay 1.0)
  (bind _outactors (Actor|GetAllActorsOfClass "/Script/Engine.TargetPoint"))
  (Components|MoveComponentTo (Variables|/Script/Engine.Actor|GetRootComponent (Game|GetPlayerCharacter 0)) (Transformation|GetActorLocation (Utilities|Array|Get(acopy) _outactors)) "0, 0, 0" false false 0.2 false)
  (Utilities|FlowControl|Delay 0.5)
  (UserInterface|Animation|PlayAnimation _oob_widget_2 (Variables|/Game/Blueprints/Widget/out_of_bounce_Widget.out_of_bounce_Widget_C|GetFadeIn _oob_widget_2) 0.0 1 "Forward" 1.0)
  (Utilities|FlowControl|Delay 1.0)
  (Variables|Default|SetStill%20TP? false)
  (Widget|RemovefromParent (Variables|Default|GetOOB_widget))
  (CallFunction|RestartBegin))

(event Custom|Restart%20Begin
  ;[0 1 0.2985] When Player Over laps OOB Box, they have 5 second to get out.
  (Utilities|FlowControl|DoOnce false) ; enters at Reset
)

(event Custom|Restart%20End
  ;[1 1 1] When Player end overlap, It will restart all vars .
  (Utilities|FlowControl|DoOnce true) ; enters at Reset
)

(fn ConstructionScript)