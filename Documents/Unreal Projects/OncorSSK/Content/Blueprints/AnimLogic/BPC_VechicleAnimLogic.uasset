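; Actor component that computes procedural wheel spin and steering transforms for a vehicle's Animation Blueprint.
; Each tick, UpdateWheelRotation derives rolling transforms from the owner's skeletal mesh sockets, wheel radius, rolling axis and previous WheelTMs.
; The first two wheels then compose WheelSteer as yaw, keeping only the resulting rotation, before WheelTMs is stored.
; Steering is fixed to yaw, as SteeringRotationAxis is unused.
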(event EventBeginPlay
  (Development|PrintString (Utilities|GetObjectName (Actor|GetComponentbyClass (Components|GetOwner) "/Script/Engine.SkeletalMeshComponent"))))

(event EventTick
  (params (DeltaSeconds :type Float%20%28single-precision%29))
  (bind _outputtms (CallFunction|UpdateWheelRotation (Actor|GetComponentbyClass (Components|GetOwner) "/Script/Engine.SkeletalMeshComponent") (Variables|Default|GetWheel%20TMs) (Variables|Default|GetSocketNames) (Variables|Default|GetWheel%20Radius) (Variables|Default|GetRollingRotationAxis))) ; Gets socket transforms, calculate wheel transform
  ;[1 1 1] Add Wheel Steer TM after Wheel Spin
  (for _index (range 0 1) ; Get first two wheels
    (Utilities|Array|SetArrayElem _outputtms _index (Math|Transform|MakeTransform (.Location (Math|Transform|BreakTransform (Utilities|Array|Get(acopy) _outputtms _index))) (.Rotation (Math|Transform|BreakTransform (Math|Transform|ComposeTransforms (Utilities|Array|Get(acopy) _outputtms _index) (Math|Conversions|ToTransform(Rotator) (Math|Rotator|MakeRotator 0.0 0.0 (Variables|Default|GetWheelSteer)))))) (.Scale (Math|Transform|BreakTransform (Utilities|Array|Get(acopy) _outputtms _index))))))
  (Variables|Default|SetWheel%20TMs _outputtms) ; TM to be used by animBP, should be set via owning Actor's blueprint, NOT the component
)