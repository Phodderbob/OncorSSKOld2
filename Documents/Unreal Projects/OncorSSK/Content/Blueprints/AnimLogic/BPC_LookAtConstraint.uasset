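; Look-at constraint scene component that computes a rotation offset toward a target actor, stored in LookAtRotation.
; Each tick, while LookAtActor is valid, it runs a LookAt along LookAtVector with Z up and takes the delta from the component's world rotation, negating roll.
; The result is relative to the component's transform, so its starting rotation matters.
; An optional debug flag draws the resulting axes at the component's location.
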(event EventBeginPlay)

(event EventTick
  (params (DeltaSeconds :type Float%20%28single-precision%29))
  (bind _returnvalue (Transformation|GetWorldTransform))
  (bind _lookat_vector (Variables|Default|GetLookAt%20Vector))
  (bind _lookat_actor (Variables|Default|GetLookAt%20Actor))
  (bind _rotation (Math|Transform|BreakTransform _returnvalue))
  (bind _returnvalue_2 (Transformation|GetActorLocation _lookat_actor))
  (bind _returnvalue_3 (Class|KismetAnimationLibrary|Lookat _returnvalue _returnvalue_2 _lookat_vector false "0.000000,0.000000,1.000000" 0.0))
  (bind _rotation_2 (Math|Transform|BreakTransform _returnvalue_3))
  (bind _returnvalue_4 (Math|Rotator|Delta(Rotator) _rotation_2 _rotation))
  (bind (_roll _pitch _yaw) (Math|Rotator|BreakRotator _returnvalue_4))
  (if (Utilities|IsValid (Variables|Default|GetLookAt%20Actor))
    (bind _output_get (Variables|Default|SetLookAt%20Rotation (Math|Rotator|MakeRotator (* _roll -1.0) _pitch _yaw)))
    (if (Variables|Default|GetDebug)
      (Class|KismetSystemLibrary|DrawDebugCoordinateSystem (Transformation|GetWorldLocation) _output_get 5e+01 0.0 0.0))))