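; Function library for procedural animation that spins wheels from socket movement and feeds a socket position to a material.
; UpdateWheelRotation runs ProcedualWheelSpin per socket against stored transforms, returning updated ones.
; Spin projects world movement onto the socket's right or forward vector, converts it through wheel circumference to degrees and accumulates on the chosen axis.
; UpdateMaterialPramFromBone writes a socket's offset bone-space X and Z into a material vector parameter.
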(fn ProcedualWheelSpin
  (params (SocketTM :type Transform) (SocketLastTm :type Transform) (WheelRadius :type Float%20%28single-precision%29) (RollingAxis :type WheelRotationAxis%20Enum :default "NewEnumerator0"))
  (bind (_location _rotation) (Math|Transform|BreakTransform SocketLastTm))
  (bind (_location_2 _rotation_2) (Math|Transform|BreakTransform SocketTM))
  ;[1 1 1] Set Local Vars
  (LocalVariables|SetCurrentLoc _location_2)
  (LocalVariables|SetLastLoc _location)
  (LocalVariables|SetCurrentRot _rotation_2)
  (LocalVariables|SetLastRot _rotation)
  (LocalVariables|SetCurrentWheelRadius WheelRadius)
  (switch Utilities|FlowControl|Switch|SwitchonWheelRotationAxis RollingAxis
    (:NewEnumerator0
      ;[1 1 1] Get position offset on Y axis - SOCKET ROTATION BREAKS DOT PRODUCT
      (LocalVariables|SetTestVal (- (LocalVariables|GetCurrentLoc) (LocalVariables|GetLastLoc)))
      (LocalVariables|SetLocChange (* (Math|Vector|VectorLength (- (LocalVariables|GetCurrentLoc) (LocalVariables|GetLastLoc))) (Math|Vector|DotProduct (Math|Vector|Normalize (- (LocalVariables|GetCurrentLoc) (LocalVariables|GetLastLoc))) (Math|Vector|GetRightVector (LocalVariables|GetCurrentRot)))))
      (return (Math|Transform|MakeTransform (LocalVariables|GetCurrentLoc) (Math|Rotator|MakeRotator (Math|Float|%(Float) (+ (* (/ (LocalVariables|GetLocChange) (* (Math|Float|MultiplybyPi 2.0) (LocalVariables|GetCurrentWheelRadius))) 3.6e+02) (.Roll (Math|Rotator|BreakRotator (LocalVariables|GetLastRot)))) 3.6e+02) 0.0 0.0))))
    (:NewEnumerator1
      ;[1 1 1] Get position offset on Y axis - SOCKET ROTATION BREAKS DOT PRODUCT
      (LocalVariables|SetTestVal (- (LocalVariables|GetCurrentLoc) (LocalVariables|GetLastLoc)))
      (LocalVariables|SetLocChange (* (Math|Vector|VectorLength (- (LocalVariables|GetCurrentLoc) (LocalVariables|GetLastLoc))) (Math|Vector|DotProduct (Math|Vector|Normalize (- (LocalVariables|GetCurrentLoc) (LocalVariables|GetLastLoc))) (Math|Vector|GetForwardVector (LocalVariables|GetCurrentRot)))))
      (return (Math|Transform|MakeTransform (LocalVariables|GetCurrentLoc) (Math|Rotator|MakeRotator 0.0 (Math|Float|%(Float) (+ (* (/ (LocalVariables|GetLocChange) (* (Math|Float|MultiplybyPi 2.0) (LocalVariables|GetCurrentWheelRadius))) 3.6e+02) (.Pitch (Math|Rotator|BreakRotator (LocalVariables|GetLastRot)))) 3.6e+02) 0.0))))
    (:NewEnumerator2
      ;[1 1 1] Get position offset on Y axis - SOCKET ROTATION BREAKS DOT PRODUCT
      (LocalVariables|SetTestVal (- (LocalVariables|GetCurrentLoc) (LocalVariables|GetLastLoc)))
      (LocalVariables|SetLocChange (* (Math|Vector|VectorLength (- (LocalVariables|GetCurrentLoc) (LocalVariables|GetLastLoc))) (Math|Vector|DotProduct (Math|Vector|Normalize (- (LocalVariables|GetCurrentLoc) (LocalVariables|GetLastLoc))) (Math|Vector|GetRightVector (LocalVariables|GetCurrentRot)))))
      (return (Math|Transform|MakeTransform (LocalVariables|GetCurrentLoc) (Math|Rotator|MakeRotator 0.0 0.0 (Math|Float|%(Float) (+ (* (/ (LocalVariables|GetLocChange) (* (Math|Float|MultiplybyPi 2.0) (LocalVariables|GetCurrentWheelRadius))) 3.6e+02) (.Yaw (Math|Rotator|BreakRotator (LocalVariables|GetLastRot)))) 3.6e+02)))))))

(fn UpdateWheelRotation
  (params (Target :type Skeletal%20Mesh%20Component%20Object%20Reference) (WheelTMs :type Array%20of%20Transforms) (SocketNames :type Array%20of%20Names) (WheelRadius :type Float%20%28single-precision%29) (RollingAxis :type WheelRotationAxis%20Enum :default "NewEnumerator0"))
  ;[1 1 1] Check arrays - Should optimize to only check on start
  (LocalVariables|SetLastWheelTM WheelTMs)
  (bind _output_get (LocalVariables|SetCurrentSocketName SocketNames))
  (if (Utilities|Array|IsValidIndex _output_get)
    (if (!= (Utilities|Array|Length (LocalVariables|GetLastWheelTM)) (Utilities|Array|Length (LocalVariables|GetCurrentSocketName)))
      (Utilities|Array|Resize (LocalVariables|GetLastWheelTM) (Utilities|Array|Length (LocalVariables|GetCurrentSocketName))))
    ;[1 1 1] Main Loop
    (for (_array_element _array_index) (LocalVariables|GetLastWheelTM) ; Loop through TM and Socket arrays
      (bind _outputtm (CallFunction|ProcedualWheelSpin (Transformation|GetSocketTransform Target (Utilities|Array|Get(acopy) (LocalVariables|GetCurrentSocketName) _array_index) "RTS_World") _array_element WheelRadius RollingAxis)) ; Compare current socket and stored TM from array, update final array
      (Utilities|Array|SetArrayElem (LocalVariables|GetNewWheelTM) _array_index _outputtm true))
    (return (LocalVariables|GetNewWheelTM))
    (else
      (Development|PrintString 0 "Socket Name variable not set yet!"))))

(fn UpdateMaterialPramfromBone
  (params (Skinned%20Mesh :type Skinned%20Mesh%20Component%20Object%20Reference) (Target%20Material :type Material%20Instance%20Dynamic%20Object%20Reference) (Material%20Pram :type Name) (Bone%20Socket :type Name) (Parent%20Bone :type Name) (Offset :type Vector))
  (bind _returnvalue (Transformation|GetSocketTransform Skinned%20Mesh Bone%20Socket "RTS_World"))
  (bind (_location _rotation) (Math|Transform|BreakTransform _returnvalue))
  (bind _outposition (Class|SkinnedMeshComponent|TransformtoBoneSpace Skinned%20Mesh Parent%20Bone _location _rotation))
  (bind _returnvalue_2 (+ _outposition Offset))
  (bind (_x _y _z) (Math|Vector|BreakVector _returnvalue_2))
  (Rendering|Material|SetVectorParameterValue Target%20Material Material%20Pram (Utilities|Struct|MakeLinearColor _x _z 0.0 1.0) :!class /Script/Engine.MaterialInstanceDynamic))