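; Stage actor that displays a player character skeletal mesh whose head tracks a LookAtPoint component.
; Construction and Tick compute a look-at rotation from the Head socket and write the remapped HeadRotation into either of two anim Blueprints.
; InitializePlayer swaps in a supplied mesh.
; ChangeToPlayer, unwired in the event graph, picks boy or girl meshes by saved TutorialCompleted and Ethnicity, with Asian girl reusing the African mesh.
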(event Custom|InitializePlayer
  (params (Mesh :type Skeletal%20Mesh%20Object%20Reference))
  (Class|SkinnedMeshComponent|SetSkeletalMesh (Variables|Default|GetSkeletalMesh) Mesh true)
  (Development|PrintString "PLAYERSTAGE!!!!!!!!!!!!" true true "(R=1.000000,G=0.457762,B=0.002988,A=1.000000)"))

(event EventBeginPlay
  ;[1 1 1] Need for ref for Save OBJ
)

(event EventTick
  (params (DeltaSeconds :type Float%20%28single-precision%29))
  (CallFunction|UpdateHeadRotation (Math|Rotator|FindLookatRotation (Transformation|GetSocketLocation (Variables|Default|GetSkeletalMesh) "Head") (Transformation|GetWorldLocation (Variables|Default|GetLookAtPoint))))
  (Variables|Default|SetTimer (+ (Variables|Default|GetTimer) DeltaSeconds)))

(fn ConstructionScript
  (Variables|Default|SetLookAtComponent (Variables|Default|GetLookAtPoint))
  (CallFunction|UpdateHeadRotation (Math|Rotator|FindLookatRotation (Transformation|GetSocketLocation (Variables|Default|GetSkeletalMesh) "Head") (Transformation|GetWorldLocation (Variables|Default|GetLookAtPoint)))))

(fn UpdateHeadRotation
  (params (Rotation :type Rotator))
  (bind (_roll _pitch _yaw) (Math|Rotator|BreakRotator Rotation))
  (bind _skeletalmesh (Variables|Default|GetSkeletalMesh))
  (bind _returnvalue (Components|SkeletalMesh|GetAnimInstance _skeletalmesh))
  (bind _asoncor_ssk_skeleton_anim_blueprint (Utilities|Casting|CastToOncor_SSK_Skeleton_AnimBlueprint _returnvalue)
    (:then
      (Variables|/Game/Models/Oncor_SSK_Skeleton_AnimBlueprint.Oncor_SSK_Skeleton_AnimBlueprint_C|SetHeadRotation _asoncor_ssk_skeleton_anim_blueprint (Math|Rotator|MakeRotator (+ (* _pitch -1.0) 9e+01) 0.0 (+ _yaw -9e+01))))
    (:CastFailed
      (bind _asoncor_ssk_adult_anim_bp (Utilities|Casting|CastToOncorSSK_Adult_AnimBP _returnvalue))
      (Variables|/Game/Models/Luis/OncorSSK_Adult_AnimBP.OncorSSK_Adult_AnimBP_C|SetHeadRotation _asoncor_ssk_adult_anim_bp (Math|Rotator|MakeRotator (+ (* _pitch -1.0) 9e+01) 0.0 (+ _yaw -9e+01))))))