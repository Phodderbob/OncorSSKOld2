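; KM_Stage is a staging actor with speaker and camera markers, hidden unless DebugDraw is on, that runs camera moves and timed actor animations.
; Lerping applies CamAnim settings, then looping 0.01-second timers simulate timelines, though Move's alpha ignores LocationTime.
; A similar timer plays queued montages when due and removes them.
; Head-look handling is an empty stub, and construction-script camera and test-actor spawning is disconnected.
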(event Custom|Lerping
  (params (came :type Camera%20Actor%20Object%20Reference) (CamAnim :type Camera%20Properties%20Structure))
  (Utilities|FlowControl|RetriggerableDelay (.timeatstart CamAnim))
  ;[1 1 1] Sets the "Vars" from Lerping
  (Variables|Lerping|SetLocationTime (.camera_location_time_to_complete CamAnim))
  (Variables|Lerping|Setstartend (.camera_location_start CamAnim))
  (Variables|Lerping|Setending (.camera_location_end CamAnim))
  (Variables|Lerping|SetCamera came)
  (Variables|Lerping|SetStartRotation (.camera_rotation_start CamAnim))
  (Variables|Lerping|SetEndRotation (.camera_rotation_end CamAnim))
  (Variables|Lerping|SetRotationTime (.camera_rotation_time_to_complete CamAnim))
  ;[1 1 1] Sets Camera Location and Rotation, current rotation Time and activate the custome events "Rotate" and "Move".
  (Transformation|SetActorLocation (Variables|Lerping|GetCamera) (Variables|Lerping|Getstartend) false false)
  (Transformation|SetActorRotation (Variables|Lerping|GetCamera) (Variables|Lerping|GetStartRotation))
  (Variables|Default|SetCurrentRotationTime (Utilities|Time|GetGameTimeinSeconds))
  (Utilities|Time|SetTimerbyFunctionName 0 "Rotate" 0.01 true)
  (Utilities|Time|SetTimerbyFunctionName 0 "Move" 0.01 true))

(event Custom|Rotate
  (bind _returnvalue (Utilities|Time|GetGameTimeinSeconds))
  ;[1 1 1] Rotates the camrea, simulating a time line.
  (if (> (Variables|Default|GetRotationTimeElapsed) (Variables|Lerping|GetRotationTime))
    (Utilities|Time|ClearTimerbyFunctionName 0 "Rotate")
    (else
      (Variables|Default|SetRotationTimeElapsed (+ (Variables|Default|GetRotationTimeElapsed) (- _returnvalue (Variables|Default|GetCurrentRotationTime))))
      (Variables|Default|SetCurrentRotationTime _returnvalue)
      (Transformation|SetActorRotation (Variables|Lerping|GetCamera) (Math|Rotator|Lerp(Rotator) (Variables|Lerping|GetStartRotation) (Variables|Lerping|GetEndRotation) (/ (Variables|Default|GetRotationTimeElapsed) (Variables|Lerping|GetRotationTime)))))))

(event Custom|StopCameraAnimation
  ;[1 1 1] Cancles the moving and roation custom event
  (Utilities|Time|ClearTimerbyFunctionName 0 "Rotate")
  (Utilities|Time|ClearTimerbyFunctionName 0 "Move"))

(event Custom|Move
  ;[1 1 1] Move the camera to a new location, simulating a timeline
  (if (> (Variables|Default|GetMovementTimeElapsed) (Variables|Lerping|GetLocationTime))
    (Utilities|Time|ClearTimerbyFunctionName 0 "Move")
    (else
      (Variables|Default|SetMovementTimeElapsed (+ (+ (Variables|Default|GetMovementTimeElapsed) (- (Variables|Default|GetMovementTimeElapsed) (Variables|Default|GetCurrentMovementTime))) 0.01))
      (Variables|Default|SetCurrentMovementTime (Variables|Default|GetMovementTimeElapsed))
      (Transformation|SetActorLocation (Variables|Lerping|GetCamera) (Math|Vector|Lerp(Vector) (Variables|Lerping|Getstartend) (Variables|Lerping|Getending) (/ (Variables|Default|GetMovementTimeElapsed) 1.0)) false false))))

(event Custom|Animation
  (bind _animations (Variables|Default|GetAnimations))
  ;[1 1 1] Move the camera to a new location, simulating a timeline
  (Variables|Default|SetAnimationTimeElapsed (+ (Variables|Default|GetAnimationTimeElapsed) 0.01))
  (for _array_element _animations
    (if (>= (Variables|Default|GetAnimationTimeElapsed) (.Time (Utilities|Struct|BreakDialogueAnimation _array_element)))
      (Animation|Montage|PlayMontage (Variables|/Game/Blueprints/StageActor.StageActor_C|GetSkeletalMesh (.ActorReference (Utilities|Struct|BreakDialogueAnimation _array_element))) (.Animation (Utilities|Struct|BreakDialogueAnimation _array_element))
        (:then
          (Utilities|Array|RemoveItem _animations _array_element))))))

(event Custom|HeadLookList
  (for _array_element (Variables|Default|GetHeadLooks)
    (if (>= (Variables|Default|GetAnimationTimeElapsed) (.Time (Utilities|Struct|BreakHeadLook_Struct _array_element)))
      (if (.IsPlayer (Utilities|Struct|BreakHeadLook_Struct _array_element))
        _))))

(event Custom|AddAnimations
  (params (Animation :type Dialogue%20Animation%20Structure))
  ;[1 1 1] Comment
  (Utilities|Array|Add (Variables|Default|GetAnimations) Animation))

(event Custom|ClearAnimations
  ;[1 1 1] Comment
  (Utilities|Time|ClearTimerbyFunctionName 0 "Animation")
  (Utilities|Time|ClearTimerbyFunctionName 0 "HeadLookList")
  (Utilities|Array|Clear (Variables|Default|GetAnimations)))

(event Custom|StartAnimatingActors
  ;[1 1 1] Comment
  (Variables|Default|SetAnimationTimeElapsed 0.0)
  (Utilities|Time|SetTimerbyFunctionName 0 "Animation" 0.01 true)
  (Utilities|Time|SetTimerbyFunctionName 0 "HeadLookList" 0.01 true))

(event EventBeginPlay
  (if (not (Variables|Default|GetDebugDraw?))
    (Rendering|SetVisibility (Variables|Default|GetStage) false false)))

(fn ConstructionScript
  (Utilities|FlowControl|Sequence
    (:then_1
      (if (Variables|Default|GetSpawnTestActors?)
        _))))