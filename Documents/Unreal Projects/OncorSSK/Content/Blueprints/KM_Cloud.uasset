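; Cloud Blueprint that slides a configurable sky mesh from a starting position between two placed points, PointA and PointB.
; Initialize places the mesh by lerping between the points with StartingPosition, in both the construction script and BeginPlay.
; BeginPlay then runs MoveComponentTo toward PointB over Time and sets the mesh back to PointA afterward, with no repeat.
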(event Custom|Initialize
  (Transformation|SetRelativeLocation (Variables|Default|GetStaticMesh) (Math|Vector|Lerp(Vector) (Variables|/Script/Engine.SceneComponent|GetRelativeLocation (Variables|Default|GetPointA)) (Variables|/Script/Engine.SceneComponent|GetRelativeLocation (Variables|Default|GetPointB)) (Variables|Default|GetStartingPosition)) false false))

(event EventBeginPlay
  (bind _staticmesh (Variables|Default|GetStaticMesh))
  (CallFunction|Initialize)
  (Components|MoveComponentTo _staticmesh (Variables|/Script/Engine.SceneComponent|GetRelativeLocation (Variables|Default|GetPointB)) "0, 0, 0" false false (Variables|Default|GetTime) false)
  (Transformation|SetRelativeLocation _staticmesh (Variables|/Script/Engine.SceneComponent|GetRelativeLocation (Variables|Default|GetPointA)) false false))

(fn ConstructionScript
  (Components|StaticMesh|SetStaticMesh (Variables|Default|GetStaticMesh) (Variables|Default|GetSkyMesh))
  (CallFunction|Initialize))