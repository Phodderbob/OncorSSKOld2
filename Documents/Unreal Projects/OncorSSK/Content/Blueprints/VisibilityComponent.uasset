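; VisibilityComponent is a component that records names marked to be visible or hidden for its owning actor.
; AddVisible and AddHidden add a name uniquely to the SetToVisible or SetToHidden array, then append it to the owner's Tags.
; Nothing here changes visibility, removes names or reconciles the two arrays.
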(event Custom|Add%20Visible
  (params (Name :type Name))
  (Utilities|Array|AddUnique (Variables|Default|GetSetToVisible) Name)
  (Utilities|Array|Add (Variables|/Script/Engine.Actor|GetTags (Components|GetOwner)) Name))

(event Custom|Add%20Hidden
  (params (Name :type Name))
  (Utilities|Array|AddUnique (Variables|Default|GetSetToHidden) Name)
  (Utilities|Array|Add (Variables|/Script/Engine.Actor|GetTags (Components|GetOwner)) Name))

(event EventBeginPlay)