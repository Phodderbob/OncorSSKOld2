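; Dialogue trigger actor that plays a conversation once and advances story progression afterwards.
; Dialogue starts on overlap, through the player's prompt, or via a Gamecontroller spawn delegate when the saved game state matches.
; SceneChange repositions the player, optionally adds a quest, then either unhides a custom level or saves its level as completed.
; The last trigger of a game state loads the next state; others unload their streamed level, and "End" wipes the save.
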(event Custom|SceneChange
  (if (Utilities|Enum|Equal(Enum) (Variables|Default|GetGS_ToLoad) "End")
    (CallFunction|ClearSave)
    (Game|OpenLevel(byName) "OncorNeighorhood")
    (else
      (Utilities|FlowControl|Sequence
        (:then_0
          ;[1 1 1] Returns control to the player
          (bind _asthird_person_character (Utilities|Casting|CastToThirdPersonCharacter (Game|Player|GetPlayerPawn 0)))
          (Default|ShowHUD _asthird_person_character)
          (Transformation|SetActorLocation _asthird_person_character (Transformation|GetWorldLocation (Variables|Default|GetRespawnPoint)) false false))
        (:then_1
          (if (Variables|Default|GetNewQuest?)
            (CallFunction|AddQuest)))
        (:then_2
          (if (Utilities|Enum|NotEqual(Enum) (Variables|Default|GetCustomLevelToUnhide) "")
            ;[1 1 1] Unhide a specific level
            (bind _outactors (Actor|GetAllActorsOfClass "/Game/Blueprints/TestFolder/gamecontroller.gamecontroller_C"))
            (for _array_element _outactors
              (Default|UnhideLevelUpdatePOI _array_element (Variables|Default|GetCustomLevelToUnhide)))
            (else
              ;[1 1 1] Finds all triggers that are in the game that matches this trigger's game state
              (Variables|Default|SetComplete true)
              (bind _outactors_2 (Actor|GetAllActorsOfClass "Trigger_C"))
              (for _array_element_2 _outactors_2
                (if (Utilities|Enum|Equal(Enum) (Variables|Trigger_C|GetGamestate _array_element_2) (Variables|Default|GetGamestate))
                  (Utilities|Array|Add (Variables|Default|GetFoundTriggers) _array_element_2)))
              ;[1 1 1] Checks to see if this i the last trigger fromt his game state
              (if (== (Utilities|Array|Length (Variables|Default|GetFoundTriggers)) 1)
                ;[1 1 1] Changes Game State
                (CallFunction|SaveLVLList)
                (Utilities|FlowControl|Delay 0.2)
                (bind _outactors_3 (Actor|GetAllActorsOfClass "/Game/Blueprints/TestFolder/gamecontroller.gamecontroller_C"))
                (for _array_element_3 _outactors_3
                  (CallFunction|SaveGameState (Variables|Default|GetGS_ToLoad))
                  ;;[1 1 1] Go to gamecontroller
                  (Default|Message _array_element_3 (Variables|Default|GetGS_ToLoad))
                  ;;[1 1 1] Music Sound Test
                  (bind _asthird_person_character_2 (Utilities|Casting|CastToThirdPersonCharacter (Game|Player|GetPlayerPawn 0)))
                  (Default|ChangeVolume _asthird_person_character_2 0.2))
                (else
                  ;[1 1 1] Unloads the Level this trigger resides in
                  (CallFunction|SaveLVLList)
                  (Utilities|FlowControl|Delay 0.2)
                  (bind _outactors_4 (Actor|GetAllActorsOfClass "/Game/Blueprints/TestFolder/gamecontroller.gamecontroller_C"))
                  (for _array_element_4 _outactors_4
                    (Default|UpdateIcons _array_element_4))
                  (Utilities|FlowControl|Delay 0.2)
                  (Game|UnloadStreamLevel(byName) (Variables|Default|GetLevel) false))))))
        (:then_3
          ;[1 1 1] If this dialogue finishes and it is Luis 1, resume the tutorial
          (if (== (Variables|Default|GetDialogueToPlay) "/Game/Blueprints/Datatables/Dialogues/Luis1.Luis1")
            _))
        (:then_4
          ;[1 1 1] Destroys this trigger
          (Utilities|FlowControl|Delay 5.0)
          (Actor|DestroyActor))))))

(event Custom|Save%20LVL%20List
  (bind _savestruct (CallFunction|GetSave))
  (bind (_gs _collectables _gender _ethnicity _languages _player_location _tutorialcompleted_ _completed_minigames _completed_lvls _currentquests) (Utilities|Struct|BreakSave_Struct _savestruct))
  ;[0.1864 0.3194 1] Save the Level Name in the Save COmpleted Lvl.s in Save Game
  (bind _output_get (Variables|Default|SetTemplLvlList (.Completed_Lvls (Utilities|Struct|BreakSave_Struct _savestruct))))
  (Utilities|Array|AddUnique _output_get (Utilities|String|ToString(Name) (Variables|Default|GetLevel)))
  (CallFunction|Save (Utilities|Struct|MakeSave_Struct _gs _collectables _gender _ethnicity _languages _player_location _tutorialcompleted_ _completed_minigames (Variables|Default|GetTemplLvlList) _currentquests 0.5 0.5)))

(event Custom|Trigger%20Dialogue
  (bind _poi_component (Variables|Default|GetPOI_Component))
  (bind _poi_component_2 (Variables|Default|GetPOI_Component))
  (bind _bp (Variables|/Game/Blueprints/POI_Component.POI_Component_C|GetBP _poi_component))
  (Utilities|FlowControl|DoOnce false
    (:Completed
      (Default|HideTextBox (.AsThird%20Person%20Character (Utilities|Casting|CastToThirdPersonCharacter (Game|Player|GetPlayerPawn 0))))
      (Utilities|IsValid _bp
        (:Is%20Valid
          (Actor|DestroyActor _bp))
        (:Is%20Not%20Valid
          _))
      (bind _outactors (Actor|GetAllActorsOfClass "/Game/Blueprints/OverHead_Icon.OverHead_Icon_C"))
      (for _array_element _outactors
        (Actor|DestroyActor _array_element))
      (Utilities|IsValid _poi_component_2
        (:Is%20Valid
          ;[1 1 1] the new changes to "Trigger" fource me to call this node here
          (Default|CallingRemoveButKeep _poi_component_2))
        (:Is%20Not%20Valid
          _))
      ;[1 1 1] Create Dialogue Widget
      (bind _returnvalue (UserInterface|CreateWidget "/Game/Blueprints/Widget/Dialogue/Dialogue.Dialogue_C" (Game|GetPlayerController 0)))
      (UserInterface|Viewport|AddtoViewport _returnvalue 0)
      (bind _asthird_person_character (Utilities|Casting|CastToThirdPersonCharacter (Game|Player|GetPlayerPawn 0)))
      (Variables|/Game/ThirdPersonBP/Blueprints/ThirdPersonCharacter.ThirdPersonCharacter_C|SetDialogue _asthird_person_character _returnvalue)
      (Variables|/Game/Blueprints/Widget/Dialogue/Dialogue.Dialogue_C|SetStage _returnvalue (Variables|Default|GetStage))
      (Variables|/Game/Blueprints/Widget/Dialogue/Dialogue.Dialogue_C|SetDialogue _returnvalue (Variables|Default|GetDialogueToPlay))
      (Variables|/Game/Blueprints/Widget/Dialogue/Dialogue.Dialogue_C|SetTrigger _returnvalue self)
      ;[1 1 1] music sound test
      (bind _asthird_person_character_2 (Utilities|Casting|CastToThirdPersonCharacter (Game|Player|GetPlayerPawn 0)))
      (Default|ChangeVolume _asthird_person_character_2 0.1)
      (Default|StartDialogue _returnvalue))))

(event Custom|AddQuest
  ;[1 1 1] Adds Quest
  (bind _asthird_person_character (Utilities|Casting|CastToThirdPersonCharacter (Game|Player|GetPlayerPawn 0)))
  (Default|ClearPrompt _asthird_person_character)
  (CallFunction|AddQuest (Utilities|Struct|MakeQuestSaveStruct (Variables|Default|GetQuest) 0 0))
  (bind _returnvalue (UserInterface|CreateWidget "/Game/Blueprints/Widget/Quest.Quest_C"))
  (Variables|/Game/Blueprints/Widget/Quest.Quest_C|SetQuestType _returnvalue (Variables|Default|GetQuest))
  (Class|VerticalBox|AddChildtoVerticalBox (Variables|/Game/Blueprints/SSK_HUD.SSK_HUD_C|GetQuestBox (Variables|/Game/ThirdPersonBP/Blueprints/ThirdPersonCharacter.ThirdPersonCharacter_C|GetHud _asthird_person_character)) _returnvalue)
  (Default|Initialize _returnvalue))

(event Custom|SpawnEvent
  (bind _poi_component (Variables|Default|GetPOI_Component))
  (bind _poi_component_2 (Variables|Default|GetPOI_Component))
  (bind _bp (Variables|/Game/Blueprints/POI_Component.POI_Component_C|GetBP _poi_component))
  (if (Utilities|Enum|Equal(Enum) (.GS (Utilities|Struct|BreakSave_Struct (.SaveStruct (CallFunction|GetSave)))) (Variables|Default|GetGamestate))
    (Utilities|FlowControl|Delay 0.2)
    (Utilities|FlowControl|DoOnce false
      (:Completed
        (Default|HideTextBox (.AsThird%20Person%20Character (Utilities|Casting|CastToThirdPersonCharacter (Game|Player|GetPlayerPawn 0))))
        (Utilities|IsValid _bp
          (:Is%20Valid
            (Actor|DestroyActor _bp))
          (:Is%20Not%20Valid
            _))
        (bind _outactors (Actor|GetAllActorsOfClass "/Game/Blueprints/OverHead_Icon.OverHead_Icon_C"))
        (for _array_element _outactors
          (Actor|DestroyActor _array_element))
        (Utilities|IsValid _poi_component_2
          (:Is%20Valid
            ;[1 1 1] the new changes to "Trigger" fource me to call this node here
            (Default|CallingRemoveButKeep _poi_component_2))
          (:Is%20Not%20Valid
            _))
        ;[1 1 1] Create Dialogue Widget
        (bind _returnvalue (UserInterface|CreateWidget "/Game/Blueprints/Widget/Dialogue/Dialogue.Dialogue_C" (Game|GetPlayerController 0)))
        (UserInterface|Viewport|AddtoViewport _returnvalue 0)
        (bind _asthird_person_character (Utilities|Casting|CastToThirdPersonCharacter (Game|Player|GetPlayerPawn 0)))
        (Variables|/Game/ThirdPersonBP/Blueprints/ThirdPersonCharacter.ThirdPersonCharacter_C|SetDialogue _asthird_person_character _returnvalue)
        (Variables|/Game/Blueprints/Widget/Dialogue/Dialogue.Dialogue_C|SetStage _returnvalue (Variables|Default|GetStage))
        (Variables|/Game/Blueprints/Widget/Dialogue/Dialogue.Dialogue_C|SetDialogue _returnvalue (Variables|Default|GetDialogueToPlay))
        (Variables|/Game/Blueprints/Widget/Dialogue/Dialogue.Dialogue_C|SetTrigger _returnvalue self)
        ;[1 1 1] music sound test
        (bind _asthird_person_character_2 (Utilities|Casting|CastToThirdPersonCharacter (Game|Player|GetPlayerPawn 0)))
        (Default|ChangeVolume _asthird_person_character_2 0.1)
        (Default|StartDialogue _returnvalue)))))

(event EventBeginPlay
  ;[1 1 1] If this dialogue is supposed to play on spawn, bind an event to the delegate on the game controller
  (bind _outactors (Actor|GetAllActorsOfClass "/Game/Blueprints/TestFolder/gamecontroller.gamecontroller_C"))
  (for _array_element _outactors
    (if (Variables|Default|Getplayonspawn)
      (EventDispatchers|BindEventtoCallPlayonSpawn _array_element (delegate Custom|SpawnEvent)))))

(event Collision|EventActorBeginOverlap
  (params (OtherActor :type Actor%20Object%20Reference))
  (bind _returnvalue (Game|Player|GetPlayerPawn 0))
  (bind _poi_component (Variables|Default|GetPOI_Component))
  (bind _poi_component_2 (Variables|Default|GetPOI_Component))
  (bind _asthird_person_character (Utilities|Casting|CastToThirdPersonCharacter _returnvalue))
  (bind _bp (Variables|/Game/Blueprints/POI_Component.POI_Component_C|GetBP _poi_component))
  (Utilities|Casting|CastToThirdPersonCharacter OtherActor)
  (if (Variables|Default|GetOverlap?)
    (Development|PrintString "DialogueOverlap")
    (Utilities|FlowControl|DoOnce false
      (:Completed
        (Default|HideTextBox _asthird_person_character)
        (Utilities|IsValid _bp
          (:Is%20Valid
            (Actor|DestroyActor _bp))
          (:Is%20Not%20Valid
            _))
        (bind _outactors (Actor|GetAllActorsOfClass "/Game/Blueprints/OverHead_Icon.OverHead_Icon_C"))
        (for _array_element _outactors
          (Actor|DestroyActor _array_element))
        (Utilities|IsValid _poi_component_2
          (:Is%20Valid
            ;[1 1 1] the new changes to "Trigger" fource me to call this node here
            (Default|CallingRemoveButKeep _poi_component_2))
          (:Is%20Not%20Valid
            _))
        ;[1 1 1] Create Dialogue Widget
        (bind _returnvalue_2 (UserInterface|CreateWidget "/Game/Blueprints/Widget/Dialogue/Dialogue.Dialogue_C" (Game|GetPlayerController 0)))
        (UserInterface|Viewport|AddtoViewport _returnvalue_2 0)
        (bind _asthird_person_character_2 (Utilities|Casting|CastToThirdPersonCharacter (Game|Player|GetPlayerPawn 0)))
        (Variables|/Game/ThirdPersonBP/Blueprints/ThirdPersonCharacter.ThirdPersonCharacter_C|SetDialogue _asthird_person_character_2 _returnvalue_2)
        (Variables|/Game/Blueprints/Widget/Dialogue/Dialogue.Dialogue_C|SetStage _returnvalue_2 (Variables|Default|GetStage))
        (Variables|/Game/Blueprints/Widget/Dialogue/Dialogue.Dialogue_C|SetDialogue _returnvalue_2 (Variables|Default|GetDialogueToPlay))
        (Variables|/Game/Blueprints/Widget/Dialogue/Dialogue.Dialogue_C|SetTrigger _returnvalue_2 self)
        ;[1 1 1] music sound test
        (bind _asthird_person_character_3 (Utilities|Casting|CastToThirdPersonCharacter (Game|Player|GetPlayerPawn 0)))
        (Default|ChangeVolume _asthird_person_character_3 0.1)
        (Default|StartDialogue _returnvalue_2)))
    (else
      ;[1 1 1] Call Show Text Box when player enters the Overlap box and send a Refrence to TPC
      (Default|ShowTextBox _asthird_person_character)
      (Default|TriggerREF _asthird_person_character self))))

(event Collision|EventActorEndOverlap
  (params (OtherActor :type Actor%20Object%20Reference))
  ;[1 1 1] Call Hide Text Box when player leave the Overlap box
  (bind _asthird_person_character (Utilities|Casting|CastToThirdPersonCharacter OtherActor))
  (Default|HideTextBox _asthird_person_character)
  (Variables|/Game/ThirdPersonBP/Blueprints/ThirdPersonCharacter.ThirdPersonCharacter_C|SetTrigger _asthird_person_character 0))

(fn ConstructionScript)