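; Stage character actor that gives child and adult characters animated faces for dialogue scenes.
; Initialize, self-triggered on static actors via a Gamecontroller event, picks the AnimBP by skeleton and can swap NPC child or mother meshes using saved player data, refreshing dialogue portraits.
; Timelines drive brow, blink and fake lip-sync, blending random phoneme poses through morph targets and jaw alpha.
; Emotion sets smile or frown; Tick aims the head at LookAtPoint.
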(event Custom|StaticInitialize
  ;[1 1 1] Need for ref for Save OBJ
  (if (Variables|Default|Getstatic?)
    (CallFunction|Initialize (Variables|Default|GetTalkingStatic) false "NewEnumerator0")))

(event Custom|Initialize
  (params (IsTalking :type Boolean) (IsPlayer :type Boolean) (Emotion :type Emotion%20Enum :default "NewEnumerator0") (Dialogue :type Dialogue%20Object%20Reference))
  (bind _savestruct (CallFunction|GetSave))
  (bind _skeletalmesh (Variables|Default|GetSkeletalMesh))
  (bind _skeletalmesh_2 (Variables|Default|GetSkeletalMesh))
  (bind _skeletalmesh_3 (Variables|Default|GetSkeletalMesh))
  (bind _ethnicity (Utilities|Struct|BreakSave_Struct _savestruct))
  (bind _skeletalmesh_4 (Variables|/Script/Engine.SkinnedMeshComponent|GetSkeletalMesh _skeletalmesh_2))
  (Variables|Default|SetDialogue Dialogue)
  (Utilities|FlowControl|Sequence
    (:then_1
      ;[1 1 1] EyebrowMovement
      (bind _alpha (Timeline|Timeline_0 PlayFromStart)
        (:Update
          (Components|SkeletalMesh|SetMorphTarget (Variables|Default|GetSkeletalMesh) "Brow Raise" _alpha true))
        (:Finished
          (Utilities|FlowControl|Delay 0.2)
          (Timeline|Timeline_0 PlayFromStart))))
    (:then_2
      (Variables|Default|SetEmotion Emotion))
    (:then_3
      (if (== (Variables|/Script/Engine.SkeletalMesh|GetSkeleton _skeletalmesh_4) "/Game/Models/Oncor_SSK_Skeleton.Oncor_SSK_Skeleton")
        (if IsPlayer
          _
          (else
            (|ChangeChildNPC _skeletalmesh_4
              (:Exec
                _))))
        (Class|SkeletalMeshComponent|SetAnimClass _skeletalmesh_2 "/Game/Models/Oncor_SSK_Skeleton_AnimBlueprint.Oncor_SSK_Skeleton_AnimBlueprint_C")
        (bind _asoncor_ssk_skeleton_anim_blueprint (Utilities|Casting|CastToOncor_SSK_Skeleton_AnimBlueprint (Components|SkeletalMesh|GetAnimInstance _skeletalmesh_2)))
        (Variables|/Game/Models/Oncor_SSK_Skeleton_AnimBlueprint.Oncor_SSK_Skeleton_AnimBlueprint_C|SetTalking _asoncor_ssk_skeleton_anim_blueprint IsTalking)
        ;[1 1 1] Blink
        (bind _alpha_2 (Timeline|Timeline_2 PlayFromStart)
          (:Update
            (Components|SkeletalMesh|SetMorphTarget (Variables|Default|GetSkeletalMesh) "Eyelid Closed" _alpha_2 true))
          (:Finished
            (Utilities|FlowControl|Delay (Math|Random|RandomFloatinRange 0.5 1.5))
            (Timeline|Timeline_2 PlayFromStart)))
        (else
          (Class|SkeletalMeshComponent|SetAnimClass _skeletalmesh_2 "/Game/Models/Luis/OncorSSK_Adult_AnimBP.OncorSSK_Adult_AnimBP_C")
          (bind _asoncor_ssk_adult_anim_bp (Utilities|Casting|CastToOncorSSK_Adult_AnimBP (Components|SkeletalMesh|GetAnimInstance _skeletalmesh_2))
            (:then
              (Variables|/Game/Models/Luis/OncorSSK_Adult_AnimBP.OncorSSK_Adult_AnimBP_C|SetTalking _asoncor_ssk_adult_anim_bp IsTalking)
              (Utilities|FlowControl|Sequence
                (:then_0
                  (if (Math|Boolean|ORBoolean (== _skeletalmesh_4 "/Game/Models/ModelsV3/Oncor_Adult_Chars/Moms/Caucasian/CaucasianMom_Rigged.CaucasianMom_Rigged") (== _skeletalmesh_4 "/Game/Models/ModelsV3/Oncor_Adult_Chars/Moms/African/AfricanMom_Rigged.AfricanMom_Rigged") (== _skeletalmesh_4 "/Game/Models/ModelsV3/Oncor_Adult_Chars/Moms/Hispanic/HispanicMom_Rigged.HispanicMom_Rigged") (== _skeletalmesh_4 "/Game/Models/ModelsV3/Oncor_Adult_Chars/Moms/Asian/AsianMom_Rigged.AsianMom_Rigged"))
                    ;[0 1 0.2985] Changes the texture of the mother depening on the player Ethnicity.
                    (if (Variables|Default|GetMatchEthnicity)
                      (switch Utilities|FlowControl|Switch|SwitchonEthnicity _ethnicity
                        (:NewEnumerator0
                          (Class|SkinnedMeshComponent|SetSkeletalMesh _skeletalmesh "/Game/Models/ModelsV3/Oncor_Adult_Chars/Moms/Caucasian/CaucasianMom_Rigged.CaucasianMom_Rigged" true :!label _label))
                        (:NewEnumerator1
                          (Class|SkinnedMeshComponent|SetSkeletalMesh _skeletalmesh "/Game/Models/ModelsV3/Oncor_Adult_Chars/Moms/African/AfricanMom_Rigged.AfricanMom_Rigged" true :!label _label_2))
                        (:NewEnumerator2
                          (Class|SkinnedMeshComponent|SetSkeletalMesh _skeletalmesh "/Game/Models/ModelsV3/Oncor_Adult_Chars/Moms/Hispanic/HispanicMom_Rigged.HispanicMom_Rigged" true))
                        (:NewEnumerator3
                          (Class|SkinnedMeshComponent|SetSkeletalMesh _skeletalmesh "/Game/Models/ModelsV3/Oncor_Adult_Chars/Moms/Asian/AsianMom_Rigged.AsianMom_Rigged" true :!label _label_3)))
                      (else
                        (switch Utilities|FlowControl|Switch|SwitchonEthnicity _ethnicity
                          (:NewEnumerator0
                            (goto _label_2))
                          (:NewEnumerator1
                            (goto _label))
                          (:NewEnumerator2
                            (goto _label_3))
                          (:NewEnumerator3
                            (goto _label_2)))))
                    (Utilities|IsValid (Variables|Default|GetDialogue)
                      (:Is%20Valid
                        (if IsTalking
                          (Utilities|FlowControl|Delay 0.1)
                          (Default|ResetPortrait (Variables|Default|GetDialogue) (Variables|/Script/Engine.SkinnedMeshComponent|GetSkeletalMesh (Variables|Default|GetSkeletalMesh))))))))
                (:then_1
                  (Timeline|Timeline_2 PlayFromStart))))
            (:CastFailed
              (Development|PrintString "AdultCastFailed"))))))
    (:then_4
      (if IsTalking
        (CallFunction|TalkingEvent)))
    (:then_6
      ;[1 1 1] Set Emotion
      (switch Utilities|FlowControl|Switch|SwitchonEmotion (Variables|Default|GetEmotion)
        (:NewEnumerator1
          (Components|SkeletalMesh|SetMorphTarget _skeletalmesh_3 "Lip Smile" 0.5 true))
        (:NewEnumerator2
          (Components|SkeletalMesh|SetMorphTarget _skeletalmesh_3 "Lip Frown" 0.5 true))))))

(event Custom|TalkingEvent
  (Utilities|FlowControl|MultiGate true true -1 :!label _label
    (:Out%200
      (Variables|Default|SetLipPart (Math|Float|MakeLiteralFloat 0.5))
      (Variables|Default|SetLipPressor (Math|Float|MakeLiteralFloat 2.0))
      (Variables|Default|SetLipStretcher (Math|Float|MakeLiteralFloat 0.4))
      (Variables|Default|SetJawAlpha (Math|Float|MakeLiteralFloat 0.5))
      ;[1 1 1] Change Phoneme Alpha
      (bind _alpha (Timeline|Timeline_1 PlayFromStart)
        (:Update
          (CallFunction|PhonemeAdjust (Math|Float|Lerp (Variables|Default|GetLipPartOld) (Variables|Default|GetLipPart) _alpha) (Math|Float|Lerp (Variables|Default|GetLipPressorOld) (Variables|Default|GetLipPressor) _alpha) (Math|Float|Lerp (Variables|Default|GetLipStretcherOld) (Variables|Default|GetLipStretcher) _alpha) (Math|Float|Lerp (Variables|Default|GetJawAlphaOld) (Variables|Default|GetJawAlpha) _alpha)))
        (:Finished
          ;[1 1 1] Sets the old values
          (Variables|Default|SetLipPartOld (Variables|Default|GetLipPart))
          (Variables|Default|SetLipPressorOld (Variables|Default|GetLipPressor))
          (Variables|Default|SetLipStretcherOld (Variables|Default|GetLipStretcher))
          (Variables|Default|SetJawAlphaOld (Variables|Default|GetJawAlpha))
          (goto _label))))
    (:Out%201
      (Variables|Default|SetLipPart (Math|Float|MakeLiteralFloat 0.5))
      (Variables|Default|SetLipPressor (Math|Float|MakeLiteralFloat 0.5))
      (Variables|Default|SetLipStretcher (Math|Float|MakeLiteralFloat 0.5))
      (Variables|Default|SetJawAlpha (Math|Float|MakeLiteralFloat 0.75))
      (Timeline|Timeline_1 PlayFromStart))
    (:Out%202
      (Variables|Default|SetLipPart (Math|Float|MakeLiteralFloat 0.5))
      (Variables|Default|SetLipPressor (Math|Float|MakeLiteralFloat 0.65))
      (Variables|Default|SetLipStretcher (Math|Float|MakeLiteralFloat 0.85))
      (Variables|Default|SetJawAlpha (Math|Float|MakeLiteralFloat 0.1))
      (Timeline|Timeline_1 PlayFromStart))
    (:Out%203
      (Variables|Default|SetLipPart (Math|Float|MakeLiteralFloat 0.5))
      (Variables|Default|SetLipPressor (Math|Float|MakeLiteralFloat 0.65))
      (Variables|Default|SetLipStretcher (Math|Float|MakeLiteralFloat 0.0))
      (Variables|Default|SetJawAlpha (Math|Float|MakeLiteralFloat 0.15))
      (Timeline|Timeline_1 PlayFromStart))
    (:Out%204
      (Variables|Default|SetLipPart (Math|Float|MakeLiteralFloat 0.5))
      (Variables|Default|SetLipPressor (Math|Float|MakeLiteralFloat 0.65))
      (Variables|Default|SetLipStretcher (Math|Float|MakeLiteralFloat 0.0))
      (Variables|Default|SetJawAlpha (Math|Float|MakeLiteralFloat 0.4))
      (Timeline|Timeline_1 PlayFromStart))
    (:Out%205
      (Variables|Default|SetLipPart (Math|Float|MakeLiteralFloat 0.6))
      (Variables|Default|SetLipPressor (Math|Float|MakeLiteralFloat 0.85))
      (Variables|Default|SetLipStretcher (Math|Float|MakeLiteralFloat 0.35))
      (Variables|Default|SetJawAlpha (Math|Float|MakeLiteralFloat 0.35))
      (Timeline|Timeline_1 PlayFromStart))
    (:Out%206
      (Variables|Default|SetLipPart (Math|Float|MakeLiteralFloat -1.0))
      (Variables|Default|SetLipPressor (Math|Float|MakeLiteralFloat -0.2))
      (Variables|Default|SetLipStretcher (Math|Float|MakeLiteralFloat -0.2))
      (Variables|Default|SetJawAlpha (Math|Float|MakeLiteralFloat 0.2))
      (Timeline|Timeline_1 PlayFromStart))
    (:Out%207
      (Variables|Default|SetLipPart (Math|Float|MakeLiteralFloat 0.36))
      (Variables|Default|SetLipPressor (Math|Float|MakeLiteralFloat -0.2))
      (Variables|Default|SetLipStretcher (Math|Float|MakeLiteralFloat -0.2))
      (Variables|Default|SetJawAlpha (Math|Float|MakeLiteralFloat 0.04))
      (Timeline|Timeline_1 PlayFromStart))
    (:Out%208
      (Variables|Default|SetLipPart (Math|Float|MakeLiteralFloat 0.7))
      (Variables|Default|SetLipPressor (Math|Float|MakeLiteralFloat 0.9))
      (Variables|Default|SetLipStretcher (Math|Float|MakeLiteralFloat -0.09))
      (Variables|Default|SetJawAlpha (Math|Float|MakeLiteralFloat 0.05))
      (Timeline|Timeline_1 PlayFromStart))
    (:Out%209
      (Variables|Default|SetLipPart (Math|Float|MakeLiteralFloat 0.7))
      (Variables|Default|SetLipPressor (Math|Float|MakeLiteralFloat 0.9))
      (Variables|Default|SetLipStretcher (Math|Float|MakeLiteralFloat -0.09))
      (Variables|Default|SetJawAlpha (Math|Float|MakeLiteralFloat 0.2))
      (Timeline|Timeline_1 PlayFromStart))))

(event EventBeginPlay
  (if (Variables|Default|Getstatic?)
    (bind _outactors (Actor|GetAllActorsOfClass "/Game/Blueprints/TestFolder/gamecontroller.gamecontroller_C"))
    (for _array_element _outactors
      (EventDispatchers|BindEventtoStaticInitialize _array_element (delegate Custom|StaticInitialize)))))

(event EventTick
  (params (DeltaSeconds :type Float%20%28single-precision%29))
  (bind _skeletalmesh (Variables|Default|GetSkeletalMesh))
  (bind _relativelocation (Variables|/Script/Engine.SceneComponent|GetRelativeLocation _skeletalmesh))
  (CallFunction|UpdateHeadRotation (Math|Conversions|RotationFromXVector (Math|Vector|GetUnitDirection(Vector) (Math|Vector|MakeVector (.x _relativelocation) (.y _relativelocation) 9e+01) (Variables|/Script/Engine.SceneComponent|GetRelativeLocation (Variables|Default|GetLookAtPoint)))))
  (Variables|Default|SetTimer (+ (Variables|Default|GetTimer) DeltaSeconds)))

(fn ConstructionScript
  (Variables|Default|SetLookAtComponent (Variables|Default|GetLookAtPoint))
  (CallFunction|UpdateHeadRotation (Math|Rotator|FindLookatRotation (Transformation|GetSocketLocation (Variables|Default|GetSkeletalMesh) "Head") (Transformation|GetWorldLocation (Variables|Default|GetLookAtPoint)))))

(fn UpdateHeadRotation
  (params (Rotation :type Rotator))
  (bind (_roll _pitch _yaw) (Math|Rotator|BreakRotator Rotation))
  (bind (_roll_2 _pitch_2 _yaw_2) (Math|Rotator|BreakRotator Rotation))
  (bind _skeletalmesh (Variables|Default|GetSkeletalMesh))
  (bind _returnvalue (Components|SkeletalMesh|GetAnimInstance _skeletalmesh))
  (bind _asoncor_ssk_skeleton_anim_blueprint (Utilities|Casting|CastToOncor_SSK_Skeleton_AnimBlueprint _returnvalue)
    (:then
      (Variables|/Game/Models/Oncor_SSK_Skeleton_AnimBlueprint.Oncor_SSK_Skeleton_AnimBlueprint_C|SetHeadRotation _asoncor_ssk_skeleton_anim_blueprint (Math|Rotator|MakeRotator _roll_2 (* _pitch_2 -1.0) (- _yaw_2 9e+01))))
    (:CastFailed
      (bind _asoncor_ssk_adult_anim_bp (Utilities|Casting|CastToOncorSSK_Adult_AnimBP _returnvalue))
      (Variables|/Game/Models/Luis/OncorSSK_Adult_AnimBP.OncorSSK_Adult_AnimBP_C|SetHeadRotation _asoncor_ssk_adult_anim_bp (Math|Rotator|MakeRotator _roll (* _pitch -1.0) (- _yaw 9e+01))))))

(fn PhonemeAdjust
  (params (Lip%20Part :type Float%20%28single-precision%29) (Lip%20Pressor :type Float%20%28single-precision%29) (LipStretcher :type Float%20%28single-precision%29) (JawAlpha :type Float%20%28single-precision%29))
  (bind _skeletalmesh (Variables|Default|GetSkeletalMesh))
  (bind _skeletalmesh_2 (Variables|Default|GetSkeletalMesh))
  (bind _returnvalue (Components|SkeletalMesh|GetAnimInstance _skeletalmesh_2))
  (bind (_asoncor_ssk_skeleton_anim_blueprint _bsuccess) (Utilities|Casting|CastToOncor_SSK_Skeleton_AnimBlueprint _returnvalue))
  (Components|SkeletalMesh|SetMorphTarget _skeletalmesh "Lip Part" Lip%20Part false)
  (Components|SkeletalMesh|SetMorphTarget _skeletalmesh "Lip Pressor" Lip%20Pressor false)
  (Components|SkeletalMesh|SetMorphTarget _skeletalmesh "Lip Stretcher" LipStretcher false)
  (if _bsuccess
    (Variables|/Game/Models/Oncor_SSK_Skeleton_AnimBlueprint.Oncor_SSK_Skeleton_AnimBlueprint_C|SetJawAlpha _asoncor_ssk_skeleton_anim_blueprint JawAlpha)
    (else
      (bind _asoncor_ssk_adult_anim_bp (Utilities|Casting|CastToOncorSSK_Adult_AnimBP _returnvalue))
      (Variables|/Game/Models/Luis/OncorSSK_Adult_AnimBP.OncorSSK_Adult_AnimBP_C|SetJawAlpha _asoncor_ssk_adult_anim_bp JawAlpha))))