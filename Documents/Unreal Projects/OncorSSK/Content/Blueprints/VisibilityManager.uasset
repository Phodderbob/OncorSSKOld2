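; VisibilityManager is an editor-time actor that registers dialogue-driven show and hide rules on actors with a VisibilityComponent.
; When Update is set, its construction script gathers those actors, scans every Dialogues data table row, then resets Update.
; Actors whose display names appear in a row's Show list receive that row name through AddVisible.
; Hide matches call AddHidden on the matched actor's owner, rather than the actor itself.
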(event EventBeginPlay)

(event Collision|EventActorBeginOverlap
  (params (OtherActor :type Actor%20Object%20Reference)))

(event EventTick
  (params (DeltaSeconds :type Float%20%28single-precision%29)))

(fn ConstructionScript
  (if (Variables|Default|GetUpdate)
    (Utilities|Array|Clear (Variables|Default|GetActors))
    (bind _outactors (Actor|GetAllActorsOfClass "/Script/Engine.Actor"))
    (for _array_element _outactors
      (Utilities|IsValid (Actor|GetComponentbyClass _array_element "/Game/Blueprints/VisibilityComponent.VisibilityComponent_C")
        (:Is%20Valid
          (Utilities|Array|Add (Variables|Default|GetActors) _array_element))))
    (for _array_element_2 (Variables|Default|GetDialogues)
      (bind _outrownames (DataTable|GetDataTableRowNames _array_element_2))
      (for _array_element_3 _outrownames
        (bind _returnvalue (Utilities|GetDataTableRow _array_element_2 _array_element_3)
          (:then
            (if (> (Utilities|Array|Length (.Show (Utilities|Struct|BreakDialogue _returnvalue))) 0)
              (for _array_element_4 (Variables|Default|GetActors)
                (if (Utilities|Array|ContainsItem (.Show (Utilities|Struct|BreakDialogue _returnvalue)) (Utilities|String|StringToName (Utilities|GetDisplayName _array_element_4)))
                  (Utilities|IsValid (Actor|GetComponentbyClass _array_element_4 "/Game/Blueprints/VisibilityComponent.VisibilityComponent_C")
                    (:Is%20Valid
                      (Default|AddVisible (Actor|GetComponentbyClass _array_element_4 "/Game/Blueprints/VisibilityComponent.VisibilityComponent_C") _array_element_3))))))
            (if (> (Utilities|Array|Length (.Hide (Utilities|Struct|BreakDialogue _returnvalue))) 0)
              (for _array_element_5 (Variables|Default|GetActors)
                (if (Utilities|Array|ContainsItem (.Hide (Utilities|Struct|BreakDialogue _returnvalue)) (Utilities|String|StringToName (Utilities|GetDisplayName _array_element_5)))
                  (Utilities|IsValid (Actor|GetComponentbyClass (Components|GetOwner _array_element_5) "/Game/Blueprints/VisibilityComponent.VisibilityComponent_C")
                    (:Is%20Valid
                      (Default|AddHidden (Actor|GetComponentbyClass (Components|GetOwner _array_element_5) "/Game/Blueprints/VisibilityComponent.VisibilityComponent_C") _array_element_3))))))))))
    (Variables|Default|SetUpdate false)))