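; KM_BranchCut is an interactive branch actor that drops when it is cut by a click.
; BeginPlay binds a Clicked event to Cut, which enables physics on the FallingBranch mesh and then calls BranchOBJ.
; The construction script applies the configurable BranchMesh to FallingBranch.
; A HiddenObjectController reference is present but unused.
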(event Custom|Cut
  (Physics|SetSimulatePhysics (Variables|Default|GetFallingBranch) true)
  (CallFunction|BranchOBJ))

(event EventBeginPlay
  (|CallParentFunction)
  (EventDispatchers|BindEventtoClicked (delegate Custom|Cut)))

(event Collision|EventActorBeginOverlap
  (params (OtherActor :type Actor%20Object%20Reference))
  (|CallParentFunction OtherActor) ; This node is disabled and will not be called.\nDrag off pins to build functionality.
)

(event EventTick
  (params (DeltaSeconds :type Float%20%28single-precision%29))
  (|CallParentFunction DeltaSeconds) ; This node is disabled and will not be called.\nDrag off pins to build functionality.
)

(fn ConstructionScript
  (|CallParentFunction)
  (Components|StaticMesh|SetStaticMesh (Variables|Default|GetFallingBranch) (Variables|Default|GetBranchMesh)))