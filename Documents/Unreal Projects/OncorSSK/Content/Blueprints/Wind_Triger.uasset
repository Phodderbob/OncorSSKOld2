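; Wind trigger actor that sweeps a box volume along a path to switch blowing on and off for the Wind_Blowing_Actors it passes.
; On BeginPlay, the Wind timeline lerps the Box's relative location between the Start and End components.
; The Box's begin and end overlap events cast the other actor to Wind_Blowing_Actor and call Blow with true or false.
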(event OnComponentEndOverlap(Box)
  (params (OverlappedComponent :type Primitive%20Component%20Object%20Reference) (OtherActor :type Actor%20Object%20Reference) (OtherComp :type Primitive%20Component%20Object%20Reference) (OtherBodyIndex :type Integer))
  (bind _aswind_blowing_actor (Utilities|Casting|CastToWind_Blowing_Actor OtherActor))
  (Default|Blow _aswind_blowing_actor false))

(event OnComponentBeginOverlap(Box)
  (params (OverlappedComponent :type Primitive%20Component%20Object%20Reference) (OtherActor :type Actor%20Object%20Reference) (OtherComp :type Primitive%20Component%20Object%20Reference) (OtherBodyIndex :type Integer) (bFromSweep :type Boolean) (SweepResult :type Hit%20Result%20Structure%20%28by%20ref%29))
  (bind _aswind_blowing_actor (Utilities|Casting|CastToWind_Blowing_Actor OtherActor))
  (Default|Blow _aswind_blowing_actor true))

(event EventBeginPlay
  (bind _alpha (Timeline|Wind Play)
    (:Update
      (Transformation|SetRelativeLocation (Variables|Default|GetBox) (Math|Vector|Lerp(Vector) (Variables|/Script/Engine.SceneComponent|GetRelativeLocation (Variables|Default|GetStart)) (Variables|/Script/Engine.SceneComponent|GetRelativeLocation (Variables|Default|GetEnd)) _alpha) false false))))

(event Collision|EventActorBeginOverlap
  (params (OtherActor :type Actor%20Object%20Reference)))

(event EventTick
  (params (DeltaSeconds :type Float%20%28single-precision%29)))

(fn ConstructionScript)