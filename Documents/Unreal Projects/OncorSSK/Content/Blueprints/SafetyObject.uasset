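; SafetyObject is a clickable actor for a hidden-object game, representing a safety item with its own mesh and message.
; The construction script applies the configured mesh, and BeginPlay binds the click handler and sets the mesh to a custom trace channel object type.
; A click passes the actor and its message to HiddenObjectController through SafetyOBJ.
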(event Custom|SafetyClicked
  (Default|SafetyOBJ (Variables|Default|GetHiddenObjectController) (Variables|Default|GetMessageOnClick) self))

(event EventBeginPlay
  (EventDispatchers|BindEventtoClicked (delegate Custom|SafetyClicked))
  (Collision|SetCollisionObjectType (Variables|Default|GetStaticMesh) "ECC_GameTraceChannel1"))

(event Collision|EventActorBeginOverlap
  (params (OtherActor :type Actor%20Object%20Reference)))

(event MouseInput|EventActorOnClicked
  (params (ButtonPressed :type Key%20Structure)))

(fn ConstructionScript
  (Components|StaticMesh|SetStaticMesh (Variables|Default|GetStaticMesh) (Variables|Default|GetMesh)))