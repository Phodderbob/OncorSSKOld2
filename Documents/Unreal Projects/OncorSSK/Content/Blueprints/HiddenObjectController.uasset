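; Controller for a hidden-object minigame that starts when the player enters its box trigger.
; It pauses and hides the character, opens a configurable menu, registers overlapping ClickableObjects and blends to a spawned camera.
; Left-click traces from the cursor to clickables, and holding right mouse orbits the controller's yaw.
; Found objects dim their menu names and are destroyed; safety-object and cone variants update their own widgets.
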(event OnComponentBeginOverlap(Box)
  (params (OverlappedComponent :type Primitive%20Component%20Object%20Reference) (OtherActor :type Actor%20Object%20Reference) (OtherComp :type Primitive%20Component%20Object%20Reference) (OtherBodyIndex :type Integer) (bFromSweep :type Boolean) (SweepResult :type Hit%20Result%20Structure%20%28by%20ref%29))
  (Utilities|FlowControl|DoOnce false
    (:Completed
      (Utilities|Casting|CastToThirdPersonCharacter OtherActor)
      (CallFunction|StartGame))))

(event Custom|StartGame
  (bind _returnvalue (Game|GetPlayerController 0))
  ;[1 1 1] Change Gmae Controlls and cast Ref. to TPC to hold all Player Controlls.
  (Input|SetInputModeGameandUI _returnvalue 0 "DoNotLock" true)
  (bind _asthird_person_character (Utilities|Casting|CastToThirdPersonCharacter (Pawn|GetControlledPawn _returnvalue)))
  (Rendering|SetActorHiddenInGame _asthird_person_character true)
  (Default|Pause _asthird_person_character)
  ;[1 1 1] HIDE HUD HERE(Mini Map and Big Map "incase Big Map is open").
  (Default|BigMap&DialogueCheck _asthird_person_character)
  (Widget|SetVisibility (Variables|/Game/Blueprints/SSK_HUD.SSK_HUD_C|GetMiniMap (Variables|/Game/ThirdPersonBP/Blueprints/ThirdPersonCharacter.ThirdPersonCharacter_C|GetHud _asthird_person_character)) "Hidden")
  ;[1 1 1] Enables input and spawns in menu
  (Input|EnableInput (Game|GetPlayerController 0))
  (bind _returnvalue_2 (UserInterface|CreateWidget (Variables|Default|GetMenuToLoad) (Game|GetPlayerController 0)))
  (bind _output_get (Variables|Default|SetHiddenObjectMenu _returnvalue_2))
  (UserInterface|Viewport|AddtoViewport _output_get 0)
  (for _array_element (Collision|GetOverlappingActors (Variables|Default|GetBounds) "/Game/Blueprints/ClickableObject.ClickableObject_C" :!class /Script/Engine.PrimitiveComponent)
    (bind _asclickable_object (Utilities|Casting|CastToClickableObject _array_element))
    (Utilities|Array|Add (Variables|Default|GetAll%20CLickable%20Obj) _asclickable_object)
    (Variables|/Game/Blueprints/ClickableObject.ClickableObject_C|SetHiddenObjectController _asclickable_object self))
  ;[1 1 1] Gets all of the hidden objects in the level and assigns the hidden object controller to it
  (for _array_element_2 (Variables|Default|GetAll%20CLickable%20Obj)
    _)
  ;[1 1 1] Pauses the third person character while we are in hidden object game mode
  (bind _outactors (Actor|GetAllActorsOfClass "/Game/ThirdPersonBP/Blueprints/ThirdPersonCharacter.ThirdPersonCharacter_C"))
  (for _array_element_3 _outactors
    (bind _asthird_person_character_2 (Utilities|Casting|CastToThirdPersonCharacter _array_element_3))
    (Default|Pause _asthird_person_character_2))
  ;[1 1 1] Spawns in the camera which is parented to the camp point
  (bind _returnvalue_3 (Game|SpawnActorfromClass "/Script/Engine.CameraActor" (Transformation|GetWorldTransform (Variables|Default|GetCamPoint)) "Undefined" 0 0))
  (Transformation|AttachComponentToComponent _returnvalue_3 (Variables|Default|GetCamPoint) "None" "SnapToTarget" "SnapToTarget" "SnapToTarget" true)
  (Game|Player|SetViewTargetwithBlend (Game|GetPlayerController 0) _returnvalue_3 0.0 "VTBlend_Linear" 0.0 false)
  (Variables|/Script/Engine.PlayerController|SetbShowMouseCursor (Game|GetPlayerController 0) true))

(event EventBeginPlay
  ;[1 1 1] Enables input and spawns in menu
)

(event Collision|EventActorBeginOverlap
  (params (OtherActor :type Actor%20Object%20Reference)))

(event EventHiddenObj
  (params (Name :type Text) (HiddenObject :type Actor%20Object%20Reference))
  (bind _all_clickable_obj (Variables|Default|GetAll%20CLickable%20Obj))
  ;[1 1 1] Found Object custom event
  (Development|PrintString "Hello")
  (bind _ashidden_object_menu (Utilities|Casting|CastToHiddenObjectMenu (Variables|Default|GetHiddenObjectMenu)))
  (for _index (range 0 (- (Class|PanelWidget|GetChildrenCount (Variables|/Game/Blueprints/HiddenObjectMenu.HiddenObjectMenu_C|GetGridPanel_22 _ashidden_object_menu)) 1))
    (bind _asobject_name (Utilities|Casting|CastToObjectName (Class|PanelWidget|GetChildat (Variables|/Game/Blueprints/HiddenObjectMenu.HiddenObjectMenu_C|GetGridPanel_22 _ashidden_object_menu) _index)))
    (if (Utilities|Enum|Equal(Enum) Name (Class|TextBlock|GetText (Variables|/Game/Blueprints/ObjectName.ObjectName_C|GetTextBlock_26 _asobject_name)))
      ;;[1 1 1] To prevent errors.
      (if (Utilities|IsValid HiddenObject)
        (Appearance|SetColorandOpacity (Variables|/Game/Blueprints/ObjectName.ObjectName_C|GetTextBlock_26 _asobject_name) (Utilities|Struct|MakeSlateColor (Utilities|Struct|MakeLinearColor (.r (.specifiedcolor (Variables|/Script/UMG.TextBlock|GetColorAndOpacity (Variables|/Game/Blueprints/ObjectName.ObjectName_C|GetTextBlock_26 _asobject_name)))) (.g (.specifiedcolor (Variables|/Script/UMG.TextBlock|GetColorAndOpacity (Variables|/Game/Blueprints/ObjectName.ObjectName_C|GetTextBlock_26 _asobject_name)))) (.b (.specifiedcolor (Variables|/Script/UMG.TextBlock|GetColorAndOpacity (Variables|/Game/Blueprints/ObjectName.ObjectName_C|GetTextBlock_26 _asobject_name)))) 0.2) (.coloruserule (Variables|/Script/UMG.TextBlock|GetColorAndOpacity (Variables|/Game/Blueprints/ObjectName.ObjectName_C|GetTextBlock_26 _asobject_name)))) :!class /Script/UMG.TextBlock)
        (Effects|SpawnEmitteratLocation "/Game/StarterContent/Particles/P_Explosion.P_Explosion" (Transformation|GetActorLocation HiddenObject))
        (Actor|DestroyActor HiddenObject))))
  ;[1 1 1] Comment
  (for _array_element _all_clickable_obj
    (if (== _array_element HiddenObject)
      (Utilities|Array|RemoveItem _all_clickable_obj _array_element)))
  ;[1 1 1] A check to see if all the clickable OBJ are gone
  (if (== (Utilities|Array|LastIndex (Variables|Default|GetAll%20CLickable%20Obj)) -1)
    (Actor|DestroyActor)
    (else
      (Development|PrintString "Not Yet" true true "(R=0.348958,G=0.301887,B=0.101726,A=1.000000)"))))

(event EventSafetyOBJ
  (params (Message :type Text) (SafetyObject :type Actor%20Object%20Reference))
  (bind _returnvalue (Game|GetPlayerController 0))
  ;[1 1 1] Displays message from safety object and removes it
  (bind _assafety_object_menu (Utilities|Casting|CastToSafetyObjectMenu (Variables|Default|GetHiddenObjectMenu)))
  (Variables|/Game/Blueprints/SafetyObjectMenu.SafetyObjectMenu_C|SetFoundSafetyObjects _assafety_object_menu (+ (Variables|/Game/Blueprints/SafetyObjectMenu.SafetyObjectMenu_C|GetFoundSafetyObjects _assafety_object_menu) 1))
  (bind _returnvalue_2 (UserInterface|CreateWidget "/Game/Blueprints/CongratsMessage.CongratsMessage_C" (Game|GetPlayerController 0)))
  (UserInterface|Viewport|AddtoViewport _returnvalue_2 0)
  (Rendering|Components|TextRender|SetText (Variables|/Game/Blueprints/CongratsMessage.CongratsMessage_C|GetMessage _returnvalue_2) Message)
  (Actor|DestroyActor SafetyObject)
  (Math|Integer|IncrementInt (Variables|Default|GetCount)
    (:%20%20
      (if (>= (Variables|Default|GetCount) (Variables|Default|GetTotal))
        (Game|Player|SetViewTargetwithBlend _returnvalue (Pawn|GetControlledPawn _returnvalue) 0.0 "VTBlend_Linear" 0.0 false)
        (Variables|/Script/Engine.PlayerController|SetbShowMouseCursor _returnvalue false)
        (Input|SetInputModeGameOnly _returnvalue)))))

(event EventCatObj
  (Development|PrintString "Meow"))

(event EventBranchOBJ
  (Development|PrintString "Cut"))

(event EventConeOBJ
  (params (Message :type Text))
  (bind _ascone_widget (Utilities|Casting|CastToConeWidget (Variables|Default|GetHiddenObjectMenu)))
  (Default|Message _ascone_widget Message))

(event Input|MouseEvents|MouseX
  (params (AxisValue :type Float%20%28single-precision%29))
  ;[1 1 1] If Orbit is true, add rotation to the object using mouse input
  (if (Variables|Default|GetOrbit?)
    (Class|Actor|AddActorWorldRotation (Math|Rotator|MakeRotator 0.0 0.0 (* AxisValue 1.5)))))

(event Input|MouseEvents|LeftMouseButton
  (params (Key :type Key%20Structure :default "None"))
  (bind _returnvalue (Game|GetPlayerController 0))
  (bind (_worldlocation _worlddirection) (Game|Player|ConvertMouseLocationToWorldSpace _returnvalue))
  (:Pressed
    (bind _outhit (Collision|LineTraceByChannel _worldlocation (+ (* _worlddirection (Variables|Default|GetGameBounds)) (Transformation|GetWorldLocation (Variables|Default|GetCamPoint))) "TraceTypeQuery1" false 0 "ForDuration"))
    (bind _asclickable_object (Utilities|Casting|CastToClickableObject (.HitActor (Collision|BreakHitResult _outhit))))
    (Default|CallClicked _asclickable_object)
    (bind _askm_cone (Utilities|Casting|CastToKM_Cone (.HitActor (Collision|BreakHitResult _outhit))))
    (Default|ClickedPosition _askm_cone (.Location (Collision|BreakHitResult _outhit)) (.Normal (Collision|BreakHitResult _outhit)))))

(event Input|MouseEvents|RightMouseButton
  (params (Key :type Key%20Structure :default "None"))
  (bind _returnvalue (Game|GetPlayerController 0))
  ;[1 1 1] Pressing right Mouse button turns orbit mode on and off allowing the player to pan around the scene
  (:Pressed
    (Variables|Default|SetOrbit? true)
    (Input|SetInputModeGameOnly _returnvalue)
    (Variables|/Script/Engine.PlayerController|SetbShowMouseCursor _returnvalue false))
  (:Released
    (Variables|Default|SetOrbit? false)
    (Variables|/Script/Engine.PlayerController|SetbShowMouseCursor _returnvalue true)
    (Input|SetInputModeGameandUI _returnvalue 0 "DoNotLock" false)))

(fn ConstructionScript)