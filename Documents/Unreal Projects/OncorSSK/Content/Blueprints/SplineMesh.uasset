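; Spline-driven actor that lays a chosen static mesh along an editable spline, deformed to follow its curve.
; The construction script adds one spline mesh component per pair of neighboring points, attached to the spline and fitted using local-space positions and tangents.
; Each segment gets the Mesh and Material variables, while MeshScale scales the Spline component itself.
; The event graph has no active logic.
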(event EventBeginPlay)

(event Collision|EventActorBeginOverlap
  (params (OtherActor :type Actor%20Object%20Reference)))

(event EventTick
  (params (DeltaSeconds :type Float%20%28single-precision%29)))

(fn ConstructionScript
  (bind _spline (Variables|Default|GetSpline))
  (bind _spline_2 (Variables|Default|GetSpline))
  (bind _returnvalue (Spline|GetNumberOfSplinePoints _spline))
  (bind _returnvalue_2 (- _returnvalue 1))
  (for _index (range 0 _returnvalue_2)
    (if (!= _index _returnvalue_2)
      (bind _returnvalue_3 (AddComponent|AddSplineMeshComponent false))
      (Transformation|AttachComponentToComponent _returnvalue_3 _spline_2 "None" "SnapToTarget" "SnapToTarget" "KeepRelative" true)
      (Components|StaticMesh|SetStaticMesh _returnvalue_3 (Variables|Default|GetMesh))
      (Transformation|SetRelativeScale3D _spline_2 (Variables|Default|GetMeshScale))
      (Rendering|Material|SetMaterial _returnvalue_3 0 (Variables|Default|GetMaterial))
      (SplineMesh|SetStartandEnd _returnvalue_3 (Spline|GetLocationatSplinePoint _spline _index "Local") (Spline|GetTangentatSplinePoint _spline _index "Local") (Spline|GetLocationatSplinePoint _spline (+ _index 1) "Local") (Spline|GetTangentatSplinePoint _spline (+ _index 1) "Local") true :!class /Script/Engine.SplineMeshComponent))))