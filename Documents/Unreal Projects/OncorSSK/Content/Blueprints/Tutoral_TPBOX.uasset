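; A tutorial trigger box that moves the player out of the house to a fixed location.
; When a ThirdPersonCharacter overlaps the box and CanLeaveHouse is set, a DoOnce gate flags ExitHouse on the character.
; It then fires TriggerDialogue on Trigger actors tagged "Tutorial" and teleports the character after a short delay.
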(event OnComponentBeginOverlap(Box)
  (params (OverlappedComponent :type Primitive%20Component%20Object%20Reference) (OtherActor :type Actor%20Object%20Reference) (OtherComp :type Primitive%20Component%20Object%20Reference) (OtherBodyIndex :type Integer) (bFromSweep :type Boolean) (SweepResult :type Hit%20Result%20Structure%20%28by%20ref%29))
  (bind _asthird_person_character (Utilities|Casting|CastToThirdPersonCharacter OtherActor))
  (if (Variables|/Game/ThirdPersonBP/Blueprints/ThirdPersonCharacter.ThirdPersonCharacter_C|GetCanLeaveHouse _asthird_person_character)
    (Utilities|FlowControl|DoOnce (Variables|/Game/ThirdPersonBP/Blueprints/ThirdPersonCharacter.ThirdPersonCharacter_C|GetTutorial%20Finish? _asthird_person_character)
      (:Completed
        (Variables|/Game/ThirdPersonBP/Blueprints/ThirdPersonCharacter.ThirdPersonCharacter_C|SetExit%20House? _asthird_person_character true)
        (bind _outactors (Actor|GetAllActorsOfClass "/Game/Blueprints/Trigger.Trigger_C"))
        (for _array_element _outactors
          (if (Utilities|Array|ContainsItem (Variables|/Script/Engine.Actor|GetTags _array_element) "Tutorial")
            (Default|TriggerDialogue _array_element)))
        (Utilities|FlowControl|Delay 1.0)
        (Transformation|Teleport _asthird_person_character "754.000000,-4361.000000,-93.000000" "0, 0, 0")))))

(event EventBeginPlay)

(event Collision|EventActorBeginOverlap
  (params (OtherActor :type Actor%20Object%20Reference)))

(event EventTick
  (params (DeltaSeconds :type Float%20%28single-precision%29)))

(fn ConstructionScript)