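; Save_Obj is a level-placed Blueprint that loads or initializes the player's save in slot "Save".
; On BeginPlay or CallSave_OBJagian, it loads an existing SSK_Save_Game, caches current quests and prints debug stats.
; Without a save, outside OncorNeighorhood, it sets a default struct and calls SaveOver without creating a save object.
; SaveOver writes progress variables and player location, preserving gender, ethnicity, language and tutorial state from SaveGame.
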(event Custom|Call%20Save_OBJ%20agian
  ;[0.9633 0.2033 1] Needed for new game.  To prevent error and bugs
  ;[1 1 1] Creates a save when player starts, this BP must be in the map.
  (bind _returnvalue (SaveGame|DoesSaveGameExist "Save"))
  (if _returnvalue
    (bind _returnvalue_2 (SaveGame|LoadGamefromSlot "Save"))
    (bind _asssk_save_game (Utilities|Casting|CastToSSK_Save_Game _returnvalue_2))
    (bind _output_get (Variables|Default|SetSaveGame _asssk_save_game))
    ;[1 1 1] Print string to check if the data ented has ben saved.
    (Variables|Default|SetCurrentQuests (.currentquests (Variables|/Game/Blueprints/SSK_Save_Game.SSK_Save_Game_C|GetSave _output_get)))
    (Development|PrintString (Utilities|String|Append " Male: " (Utilities|String|ToString(Boolean) (.gender (Variables|/Game/Blueprints/SSK_Save_Game.SSK_Save_Game_C|GetSave _output_get))) " , " (Utilities|String|EnumtoString (.ethnicity (Variables|/Game/Blueprints/SSK_Save_Game.SSK_Save_Game_C|GetSave _output_get))) " & " (Utilities|String|EnumtoString (.languages (Variables|/Game/Blueprints/SSK_Save_Game.SSK_Save_Game_C|GetSave _output_get)))) true true "(R=0.924739,G=1.000000,B=0.151697,A=1.000000)" 5.0)
    (Development|PrintString (Utilities|String|Append "Coll: " (Utilities|String|ToString(Integer) (Utilities|Array|Length (.collectables (Variables|/Game/Blueprints/SSK_Save_Game.SSK_Save_Game_C|GetSave _output_get))))) true true "(R=1.000000,G=0.084755,B=0.265081,A=1.000000)")
    (Development|PrintString (Utilities|String|Append "Lvl.'s: " (Utilities|String|ToString(Integer) (Utilities|Array|Length (.completed_lvls (Variables|/Game/Blueprints/SSK_Save_Game.SSK_Save_Game_C|GetSave _output_get))))) true true "(R=0.000000,G=1.000000,B=0.298514,A=1.000000)")
    (Development|PrintString (Utilities|String|Append "Tutorial COmplted? " (Utilities|String|ToString(Boolean) (.tutorialcompleted? (Variables|/Game/Blueprints/SSK_Save_Game.SSK_Save_Game_C|GetSave _output_get)))) true true "(R=0.967060,G=1.000000,B=0.989879,A=1.000000)")
    (else
      (bind _returnvalue_3 (Game|GetCurrentLevelName true))
      (if (not (Utilities|Enum|Equal(Enum) _returnvalue_3 "OncorNeighorhood"))
        (Variables|Default|SetsaveStruct (Utilities|Struct|MakeSave_Struct "GS_4" (Utilities|Array|MakeArray "") true "NewEnumerator0" "NewEnumerator0" "0, 0, 0" true (Utilities|Array|MakeArray "0, 0, 0") (Utilities|Array|MakeArray "") (Utilities|Array|MakeArray (Utilities|Struct|MakeQuestSaveStruct "NewEnumerator6" 0 0)) 0.5 0.5))
        (CallFunction|SaveOver)))))

(event EventBeginPlay
  ;[1 1 1] Creates a save when player starts, this BP must be in the map.
  (bind _returnvalue (SaveGame|DoesSaveGameExist "Save"))
  (if _returnvalue
    (bind _returnvalue_2 (SaveGame|LoadGamefromSlot "Save"))
    (bind _asssk_save_game (Utilities|Casting|CastToSSK_Save_Game _returnvalue_2))
    (bind _output_get (Variables|Default|SetSaveGame _asssk_save_game))
    ;[1 1 1] Print string to check if the data ented has ben saved.
    (Variables|Default|SetCurrentQuests (.currentquests (Variables|/Game/Blueprints/SSK_Save_Game.SSK_Save_Game_C|GetSave _output_get)))
    (Development|PrintString (Utilities|String|Append " Male: " (Utilities|String|ToString(Boolean) (.gender (Variables|/Game/Blueprints/SSK_Save_Game.SSK_Save_Game_C|GetSave _output_get))) " , " (Utilities|String|EnumtoString (.ethnicity (Variables|/Game/Blueprints/SSK_Save_Game.SSK_Save_Game_C|GetSave _output_get))) " & " (Utilities|String|EnumtoString (.languages (Variables|/Game/Blueprints/SSK_Save_Game.SSK_Save_Game_C|GetSave _output_get)))) true true "(R=0.924739,G=1.000000,B=0.151697,A=1.000000)" 5.0)
    (Development|PrintString (Utilities|String|Append "Coll: " (Utilities|String|ToString(Integer) (Utilities|Array|Length (.collectables (Variables|/Game/Blueprints/SSK_Save_Game.SSK_Save_Game_C|GetSave _output_get))))) true true "(R=1.000000,G=0.084755,B=0.265081,A=1.000000)")
    (Development|PrintString (Utilities|String|Append "Lvl.'s: " (Utilities|String|ToString(Integer) (Utilities|Array|Length (.completed_lvls (Variables|/Game/Blueprints/SSK_Save_Game.SSK_Save_Game_C|GetSave _output_get))))) true true "(R=0.000000,G=1.000000,B=0.298514,A=1.000000)")
    (Development|PrintString (Utilities|String|Append "Tutorial COmplted? " (Utilities|String|ToString(Boolean) (.tutorialcompleted? (Variables|/Game/Blueprints/SSK_Save_Game.SSK_Save_Game_C|GetSave _output_get)))) true true "(R=0.967060,G=1.000000,B=0.989879,A=1.000000)")
    (else
      (bind _returnvalue_3 (Game|GetCurrentLevelName true))
      (if (not (Utilities|Enum|Equal(Enum) _returnvalue_3 "OncorNeighorhood"))
        (Variables|Default|SetsaveStruct (Utilities|Struct|MakeSave_Struct "GS_4" (Utilities|Array|MakeArray "") true "NewEnumerator0" "NewEnumerator0" "0, 0, 0" true (Utilities|Array|MakeArray "0, 0, 0") (Utilities|Array|MakeArray "") (Utilities|Array|MakeArray (Utilities|Struct|MakeQuestSaveStruct "NewEnumerator6" 0 0)) 0.5 0.5))
        (CallFunction|SaveOver)))))

(fn ConstructionScript)

(fn SaveOver
  (bind _savegame (Variables|Default|GetSaveGame))
  (bind _asthird_person_character (Utilities|Casting|CastToThirdPersonCharacter (Game|GetPlayerCharacter 0)))
  (bind _output_get (Variables|/Game/Blueprints/SSK_Save_Game.SSK_Save_Game_C|SetSave _savegame (Utilities|Struct|MakeSave_Struct (Variables|Default|GetGS%20name) (Variables|Default|GetColl_List) (.Gender (Utilities|Struct|BreakSave_Struct (Variables|/Game/Blueprints/SSK_Save_Game.SSK_Save_Game_C|GetSave (Variables|Default|GetSaveGame)))) (.Ethnicity (Utilities|Struct|BreakSave_Struct (Variables|/Game/Blueprints/SSK_Save_Game.SSK_Save_Game_C|GetSave (Variables|Default|GetSaveGame)))) (.Languages (Utilities|Struct|BreakSave_Struct (Variables|/Game/Blueprints/SSK_Save_Game.SSK_Save_Game_C|GetSave (Variables|Default|GetSaveGame)))) (Transformation|GetActorLocation _asthird_person_character) (.TutorialCompleted? (Utilities|Struct|BreakSave_Struct (Variables|/Game/Blueprints/SSK_Save_Game.SSK_Save_Game_C|GetSave (Variables|Default|GetSaveGame)))) (Variables|Default|GetVertexList) (Variables|Default|GetLvl_List) (Variables|Default|GetCurrentQuests) 0.5 0.5)))
  (bind _returnvalue (SaveGame|SaveGametoSlot _savegame "Save"))
  (Variables|Default|SetsaveStruct _output_get)
  (if _returnvalue
    (Development|PrintString (Utilities|String|ToString(Boolean) _returnvalue))
    (else
      (Development|PrintString (Utilities|String|ToString(Boolean) _returnvalue)))))