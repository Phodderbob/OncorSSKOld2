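; Muscle car Blueprint that animates steering and per-wheel offsets in response to a WheelEvent.
; The event's steering direction blends the anim blueprint's Steering toward full right, full left or straight.
; It then blends the selected wheel's offset variable toward the supplied vector.
; Each case has its own timeline that lerps from the value captured at the start, writing directly to the skeletal mesh's anim instance.
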(event Custom|WheelEvent
  (params (WheelEvent :type Wheel%20Event%20Structure))
  (bind _skeletalmeshcomponent (Variables|SkeletalMeshActor|GetSkeletalMeshComponent))
  (bind _returnvalue (Components|SkeletalMesh|GetAnimInstance _skeletalmeshcomponent))
  (Utilities|FlowControl|Sequence
    (:then_0
      (switch Utilities|FlowControl|Switch|SwitchonTurnDirection (.steeringdirection WheelEvent)
        (:NewEnumerator0
          (bind _assk_veh_car_muscle_01_skeleton_anim_blueprint (Utilities|Casting|CastToSK_Veh_Car_Muscle_01_Skeleton_AnimBlueprint _returnvalue))
          (Variables|Default|SetCurrentSteering (Variables|/Game/PolygonCity/Meshes/Vehicles_Rigged/SK_Veh_Car_Muscle_01_Skeleton_AnimBlueprint.SK_Veh_Car_Muscle_01_Skeleton_AnimBlueprint_C|GetSteering _assk_veh_car_muscle_01_skeleton_anim_blueprint))
          (bind _newtrack_0 (Timeline|Timeline_0 PlayFromStart)
            (:Update
              (Variables|/Game/PolygonCity/Meshes/Vehicles_Rigged/SK_Veh_Car_Muscle_01_Skeleton_AnimBlueprint.SK_Veh_Car_Muscle_01_Skeleton_AnimBlueprint_C|SetSteering _assk_veh_car_muscle_01_skeleton_anim_blueprint (Math|Float|Lerp (Variables|Default|GetCurrentSteering) 45.0 _newtrack_0)))))
        (:NewEnumerator1
          (bind _assk_veh_car_muscle_01_skeleton_anim_blueprint_2 (Utilities|Casting|CastToSK_Veh_Car_Muscle_01_Skeleton_AnimBlueprint _returnvalue))
          (Variables|Default|SetCurrentSteering (Variables|/Game/PolygonCity/Meshes/Vehicles_Rigged/SK_Veh_Car_Muscle_01_Skeleton_AnimBlueprint.SK_Veh_Car_Muscle_01_Skeleton_AnimBlueprint_C|GetSteering _assk_veh_car_muscle_01_skeleton_anim_blueprint_2))
          (bind _newtrack_0_2 (Timeline|Timeline_1 PlayFromStart)
            (:Update
              (Variables|/Game/PolygonCity/Meshes/Vehicles_Rigged/SK_Veh_Car_Muscle_01_Skeleton_AnimBlueprint.SK_Veh_Car_Muscle_01_Skeleton_AnimBlueprint_C|SetSteering _assk_veh_car_muscle_01_skeleton_anim_blueprint_2 (Math|Float|Lerp (Variables|Default|GetCurrentSteering) -45.0 _newtrack_0_2)))))
        (:NewEnumerator2
          (bind _assk_veh_car_muscle_01_skeleton_anim_blueprint_3 (Utilities|Casting|CastToSK_Veh_Car_Muscle_01_Skeleton_AnimBlueprint _returnvalue))
          (Variables|Default|SetCurrentSteering (Variables|/Game/PolygonCity/Meshes/Vehicles_Rigged/SK_Veh_Car_Muscle_01_Skeleton_AnimBlueprint.SK_Veh_Car_Muscle_01_Skeleton_AnimBlueprint_C|GetSteering _assk_veh_car_muscle_01_skeleton_anim_blueprint_3))
          (bind _newtrack_0_3 (Timeline|Timeline_2 PlayFromStart)
            (:Update
              (Variables|/Game/PolygonCity/Meshes/Vehicles_Rigged/SK_Veh_Car_Muscle_01_Skeleton_AnimBlueprint.SK_Veh_Car_Muscle_01_Skeleton_AnimBlueprint_C|SetSteering _assk_veh_car_muscle_01_skeleton_anim_blueprint_3 (Math|Float|Lerp (Variables|Default|GetCurrentSteering) 0.0 _newtrack_0_3)))))))
    (:then_1
      (bind _assk_veh_car_muscle_01_skeleton_anim_blueprint_4 (Utilities|Casting|CastToSK_Veh_Car_Muscle_01_Skeleton_AnimBlueprint (Components|SkeletalMesh|GetAnimInstance (Variables|SkeletalMeshActor|GetSkeletalMeshComponent))))
      (switch Utilities|FlowControl|Switch|SwitchonWheelToOffset (.wheeltooffset WheelEvent)
        (:NewEnumerator0
          (Variables|Default|SetCurrentOffset (Variables|/Game/PolygonCity/Meshes/Vehicles_Rigged/SK_Veh_Car_Muscle_01_Skeleton_AnimBlueprint.SK_Veh_Car_Muscle_01_Skeleton_AnimBlueprint_C|GetFLOffset _assk_veh_car_muscle_01_skeleton_anim_blueprint_4))
          (bind _newtrack_0_4 (Timeline|Timeline_3 PlayFromStart)
            (:Update
              (Variables|/Game/PolygonCity/Meshes/Vehicles_Rigged/SK_Veh_Car_Muscle_01_Skeleton_AnimBlueprint.SK_Veh_Car_Muscle_01_Skeleton_AnimBlueprint_C|SetFLOffset _assk_veh_car_muscle_01_skeleton_anim_blueprint_4 (Math|Vector|Lerp(Vector) (Variables|Default|GetCurrentOffset) (.wheeloffset WheelEvent) _newtrack_0_4)))))
        (:NewEnumerator1
          (Variables|Default|SetCurrentOffset (Variables|/Game/PolygonCity/Meshes/Vehicles_Rigged/SK_Veh_Car_Muscle_01_Skeleton_AnimBlueprint.SK_Veh_Car_Muscle_01_Skeleton_AnimBlueprint_C|GetFROffset _assk_veh_car_muscle_01_skeleton_anim_blueprint_4))
          (bind _newtrack_0_5 (Timeline|Timeline_4 PlayFromStart)
            (:Update
              (Variables|/Game/PolygonCity/Meshes/Vehicles_Rigged/SK_Veh_Car_Muscle_01_Skeleton_AnimBlueprint.SK_Veh_Car_Muscle_01_Skeleton_AnimBlueprint_C|SetFROffset _assk_veh_car_muscle_01_skeleton_anim_blueprint_4 (Math|Vector|Lerp(Vector) (Variables|Default|GetCurrentOffset) (.wheeloffset WheelEvent) _newtrack_0_5)))))
        (:NewEnumerator2
          (Variables|Default|SetCurrentOffset (Variables|/Game/PolygonCity/Meshes/Vehicles_Rigged/SK_Veh_Car_Muscle_01_Skeleton_AnimBlueprint.SK_Veh_Car_Muscle_01_Skeleton_AnimBlueprint_C|GetBLOffset _assk_veh_car_muscle_01_skeleton_anim_blueprint_4))
          (bind _newtrack_0_6 (Timeline|Timeline_5 PlayFromStart)
            (:Update
              (Variables|/Game/PolygonCity/Meshes/Vehicles_Rigged/SK_Veh_Car_Muscle_01_Skeleton_AnimBlueprint.SK_Veh_Car_Muscle_01_Skeleton_AnimBlueprint_C|SetBLOffset _assk_veh_car_muscle_01_skeleton_anim_blueprint_4 (Math|Vector|Lerp(Vector) (Variables|Default|GetCurrentOffset) (.wheeloffset WheelEvent) _newtrack_0_6)))))
        (:NewEnumerator3
          (Variables|Default|SetCurrentOffset (Variables|/Game/PolygonCity/Meshes/Vehicles_Rigged/SK_Veh_Car_Muscle_01_Skeleton_AnimBlueprint.SK_Veh_Car_Muscle_01_Skeleton_AnimBlueprint_C|GetBROffset _assk_veh_car_muscle_01_skeleton_anim_blueprint_4))
          (bind _newtrack_0_7 (Timeline|Timeline_6 PlayFromStart)
            (:Update
              (Variables|/Game/PolygonCity/Meshes/Vehicles_Rigged/SK_Veh_Car_Muscle_01_Skeleton_AnimBlueprint.SK_Veh_Car_Muscle_01_Skeleton_AnimBlueprint_C|SetBROffset _assk_veh_car_muscle_01_skeleton_anim_blueprint_4 (Math|Vector|Lerp(Vector) (Variables|Default|GetCurrentOffset) (.wheeloffset WheelEvent) _newtrack_0_7)))))))))

(event EventBeginPlay)

(event Collision|EventActorBeginOverlap
  (params (OtherActor :type Actor%20Object%20Reference)))

(event EventTick
  (params (DeltaSeconds :type Float%20%28single-precision%29)))

(fn ConstructionScript)