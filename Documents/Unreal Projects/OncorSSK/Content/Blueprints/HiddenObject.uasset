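; Clickable hidden object actor for a find-the-object game.
; Its construction script applies a configurable mesh to the static mesh component.
; On begin play it binds a click handler and moves the mesh to a custom collision object channel.
; When clicked, it reports its name and itself to the hidden object controller.
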(event Custom|ObjectClicked
  (Default|HiddenObj (Variables|Default|GetHiddenObjectController) (Variables|Default|GetName) self))

(event EventBeginPlay
  (EventDispatchers|BindEventtoClicked (delegate Custom|ObjectClicked))
  (Collision|SetCollisionObjectType (Variables|Default|GetStaticMesh) "ECC_GameTraceChannel1"))

(event Collision|EventActorBeginOverlap
  (params (OtherActor :type Actor%20Object%20Reference)))

(fn ConstructionScript
  (Components|StaticMesh|SetStaticMesh (Variables|Default|GetStaticMesh) (Variables|Default|GetMesh)))