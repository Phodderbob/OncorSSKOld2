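; Test actor that animates a face with random, continuous phoneme mouth shapes; no audio drives it.
; On BeginPlay it applies an Emotion smile or frown morph and starts a repeating eyebrow raise.
; A looping random MultiGate picks phoneme targets, which the MouthMove timeline blends via PhonemeAdjust into lip morph targets and the AnimBP's JawAlpha.
; JawAlphaOld assigns to itself, so jaw blends never start from the previous pose.
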(event EventBeginPlay
  (bind _skeletalmesh (Variables|Default|GetSkeletalMesh))
  (Utilities|FlowControl|Sequence
    (:then_0
      (switch Utilities|FlowControl|Switch|SwitchonEmotion (Variables|Default|GetEmotion)
        (:NewEnumerator0
          _)
        (:NewEnumerator1
          (Components|SkeletalMesh|SetMorphTarget _skeletalmesh "Lip Smile" 0.5 true))
        (:NewEnumerator2
          (Components|SkeletalMesh|SetMorphTarget _skeletalmesh "Lip Frown" 0.5 true)))
      (Utilities|FlowControl|MultiGate true true -1 :!label _label
        (:Out%200
          (Variables|Default|SetLipPart (Math|Float|MakeLiteralFloat 0.5))
          (Variables|Default|SetLipPressor (Math|Float|MakeLiteralFloat 2.0))
          (Variables|Default|SetLipStretcher (Math|Float|MakeLiteralFloat 0.4))
          (Variables|Default|SetJawAlpha (Math|Float|MakeLiteralFloat 0.5))
          (bind _alpha (Timeline|MouthMove PlayFromStart)
            (:Update
              (CallFunction|PhonemeAdjust (Math|Float|Lerp (Variables|Default|GetLipPartOld) (Variables|Default|GetLipPart) _alpha) (Math|Float|Lerp (Variables|Default|GetLipPressorOld) (Variables|Default|GetLipPressor) _alpha) (Math|Float|Lerp (Variables|Default|GetLipStretcherOld) (Variables|Default|GetLipStretcher) _alpha) (Math|Float|Lerp (Variables|Default|GetJawAlphaOld) (Variables|Default|GetJawAlpha) _alpha)))
            (:Finished
              (Variables|Default|SetLipPartOld (Variables|Default|GetLipPart))
              (Variables|Default|SetLipPressorOld (Variables|Default|GetLipPressor))
              (Variables|Default|SetLipStretcherOld (Variables|Default|GetLipStretcher))
              (Variables|Default|SetJawAlphaOld (Variables|Default|GetJawAlphaOld))
              (goto _label))))
        (:Out%201
          (Variables|Default|SetLipPart (Math|Float|MakeLiteralFloat 0.5))
          (Variables|Default|SetLipPressor (Math|Float|MakeLiteralFloat 0.5))
          (Variables|Default|SetLipStretcher (Math|Float|MakeLiteralFloat 0.5))
          (Variables|Default|SetJawAlpha (Math|Float|MakeLiteralFloat 0.75))
          (Timeline|MouthMove PlayFromStart))
        (:Out%202
          (Variables|Default|SetLipPart (Math|Float|MakeLiteralFloat 0.5))
          (Variables|Default|SetLipPressor (Math|Float|MakeLiteralFloat 0.65))
          (Variables|Default|SetLipStretcher (Math|Float|MakeLiteralFloat 0.85))
          (Variables|Default|SetJawAlpha (Math|Float|MakeLiteralFloat 0.1))
          (Timeline|MouthMove PlayFromStart))
        (:Out%203
          (Variables|Default|SetLipPart (Math|Float|MakeLiteralFloat 0.5))
          (Variables|Default|SetLipPressor (Math|Float|MakeLiteralFloat 0.65))
          (Variables|Default|SetLipStretcher (Math|Float|MakeLiteralFloat 0.0))
          (Variables|Default|SetJawAlpha (Math|Float|MakeLiteralFloat 0.15))
          (Timeline|MouthMove PlayFromStart))
        (:Out%204
          (Variables|Default|SetLipPart (Math|Float|MakeLiteralFloat 0.5))
          (Variables|Default|SetLipPressor (Math|Float|MakeLiteralFloat 0.65))
          (Variables|Default|SetLipStretcher (Math|Float|MakeLiteralFloat 0.0))
          (Variables|Default|SetJawAlpha (Math|Float|MakeLiteralFloat 0.4))
          (Timeline|MouthMove PlayFromStart))
        (:Out%205
          (Variables|Default|SetLipPart (Math|Float|MakeLiteralFloat 0.6))
          (Variables|Default|SetLipPressor (Math|Float|MakeLiteralFloat 0.85))
          (Variables|Default|SetLipStretcher (Math|Float|MakeLiteralFloat 0.35))
          (Variables|Default|SetJawAlpha (Math|Float|MakeLiteralFloat 0.35))
          (Timeline|MouthMove PlayFromStart))
        (:Out%206
          (Variables|Default|SetLipPart (Math|Float|MakeLiteralFloat -1.0))
          (Variables|Default|SetLipPressor (Math|Float|MakeLiteralFloat -0.2))
          (Variables|Default|SetLipStretcher (Math|Float|MakeLiteralFloat -0.2))
          (Variables|Default|SetJawAlpha (Math|Float|MakeLiteralFloat 0.2))
          (Timeline|MouthMove PlayFromStart))
        (:Out%207
          (Variables|Default|SetLipPart (Math|Float|MakeLiteralFloat 0.36))
          (Variables|Default|SetLipPressor (Math|Float|MakeLiteralFloat -0.2))
          (Variables|Default|SetLipStretcher (Math|Float|MakeLiteralFloat -0.2))
          (Variables|Default|SetJawAlpha (Math|Float|MakeLiteralFloat 0.04))
          (Timeline|MouthMove PlayFromStart))
        (:Out%208
          (Variables|Default|SetLipPart (Math|Float|MakeLiteralFloat 0.7))
          (Variables|Default|SetLipPressor (Math|Float|MakeLiteralFloat 0.9))
          (Variables|Default|SetLipStretcher (Math|Float|MakeLiteralFloat -0.09))
          (Variables|Default|SetJawAlpha (Math|Float|MakeLiteralFloat 0.05))
          (Timeline|MouthMove PlayFromStart))
        (:Out%209
          (Variables|Default|SetLipPart (Math|Float|MakeLiteralFloat 0.7))
          (Variables|Default|SetLipPressor (Math|Float|MakeLiteralFloat 0.9))
          (Variables|Default|SetLipStretcher (Math|Float|MakeLiteralFloat -0.09))
          (Variables|Default|SetJawAlpha (Math|Float|MakeLiteralFloat 0.2))
          (Timeline|MouthMove PlayFromStart))))
    (:then_1
      (bind _alpha_2 (Timeline|Eyebrow PlayFromStart)
        (:Update
          (Components|SkeletalMesh|SetMorphTarget (Variables|Default|GetSkeletalMesh) "Brow Raise" _alpha_2 true))
        (:Finished
          (Utilities|FlowControl|Delay 0.2)
          (Timeline|Eyebrow PlayFromStart))))))

(event Collision|EventActorBeginOverlap
  (params (OtherActor :type Actor%20Object%20Reference)))

(event EventTick
  (params (DeltaSeconds :type Float%20%28single-precision%29)))

(fn ConstructionScript)

(fn PhonemeAdjust
  (params (LipPart :type Float%20%28single-precision%29) (LipPressor :type Float%20%28single-precision%29) (LipStretcher :type Float%20%28single-precision%29) (JawAlpha :type Float%20%28single-precision%29))
  (bind _skeletalmesh (Variables|Default|GetSkeletalMesh))
  (Components|SkeletalMesh|SetMorphTarget _skeletalmesh "Lip Part" LipPart false)
  (Components|SkeletalMesh|SetMorphTarget _skeletalmesh "Lip Pressor" LipPressor false)
  (Components|SkeletalMesh|SetMorphTarget _skeletalmesh "Lip Stretcher" LipStretcher false)
  (Variables|/Game/Models/Oncor_SSK_Skeleton_AnimBlueprint.Oncor_SSK_Skeleton_AnimBlueprint_C|SetJawAlpha (.AsOncor%20SSK%20Skeleton%20Anim%20Blueprint (Utilities|Casting|CastToOncor_SSK_Skeleton_AnimBlueprint (Components|SkeletalMesh|GetAnimInstance (Variables|Default|GetSkeletalMesh)))) JawAlpha))