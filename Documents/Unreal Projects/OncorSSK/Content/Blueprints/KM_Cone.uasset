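; Cone-placement mini-game that spawns up to five cones at clicked positions and judges the layout once the fifth is placed.
; Cones fail if any overlaps InnerRing, not all five overlap OuterRing, or any pair is under a minimum spacing.
; Failures trigger a delayed clear of cones; results reach HiddenObjectController through OncorSSKInterface actors.
; The spacing failure message says "too far apart", and the success message still follows that failure.
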(event Custom|AddConeCount
  ;[1 1 1] Add 1 cone and set the count after clicking the play area
  (Variables|Default|SetConeCount (+ (Variables|Default|GetConeCount) 1)))

(event Custom|Reset
  (bind _conearray (Variables|Default|GetConeArray))
  ;[1 1 1] Process for bringing up a dialog for success or failure, then resetting the cones if mini-game has failed.
  (Utilities|FlowControl|Delay 1.0)
  (Development|PrintString "Reset!")
  (for _array_element _conearray
    (Actor|DestroyActor _array_element))
  (Utilities|Array|Clear _conearray)
  (Variables|Default|SetConeCount 0))

(event Custom|SendMessage
  (params (Message :type Text))
  ;[1 1 1] Text message based on success or failure
  (bind _outactors (Actor|GetAllActorswithInterface "/Game/Blueprints/OncorSSKInterface.OncorSSKInterface_C"))
  (for _array_element _outactors
    (bind _ashidden_object_controller (Utilities|Casting|CastToHiddenObjectController _array_element))
    (Default|ConeOBJ _ashidden_object_controller Message)))

(event EventClickedPosition
  (params (Position :type Vector :default "0, 0, 0") (Normal :type Vector :default "0, 0, 0"))
  (bind _outerring (Variables|Default|GetOuterRing))
  (bind _overlappingactors (Collision|GetOverlappingActors _outerring "/Game/Blueprints/Cone.Cone_C" :!class /Script/Engine.PrimitiveComponent))
  ;[1 1 1] As long as cone count is less than 5, spawn a cone mesh
  (Development|PrintString "Cone")
  (if (< (Variables|Default|GetConeCount) 5)
    (CallFunction|AddConeCount)
    (bind _returnvalue (Game|SpawnActorfromClass "/Game/Blueprints/Cone.Cone_C" (Math|Transform|MakeTransform Position "0, 0, 0" "1,1,1") "Undefined" 0 0))
    ;[1 1 1] Add cones to the array until 5 are placed
    (Utilities|Array|Add (Variables|Default|GetConeArray) _returnvalue)
    (if (== (Variables|Default|GetConeCount) 5)
      ;[1 1 1] Reset conditions based on incorrect amount of cones or improper placements (and matching messages)
      (if (> (Utilities|Array|Length (Collision|GetOverlappingActors (Variables|Default|GetInnerRing) "/Game/Blueprints/Cone.Cone_C" :!class /Script/Engine.PrimitiveComponent)) 0)
        (CallFunction|Reset)
        (CallFunction|SendMessage "Failure! A cone was in the center.")
        (elif (!= (Utilities|Array|Length (Collision|GetOverlappingActors (Variables|Default|GetOuterRing) "/Game/Blueprints/Cone.Cone_C" :!class /Script/Engine.PrimitiveComponent)) 5)
          (CallFunction|Reset)
          (CallFunction|SendMessage "Failure! Try placing cones closer to the target.")
          (else
            (bind _array_element (Utilities|Array|ForEachLoopwithBreak _overlappingactors :!label _label)
              (:LoopBody
                (for _array_element_2 _overlappingactors
                  (if (!= _array_element _array_element_2)
                    (if (< (Math|Vector|VectorLength (- (Transformation|GetActorLocation _array_element) (Transformation|GetActorLocation _array_element_2))) 1e+02)
                      (CallFunction|Reset)
                      (CallFunction|SendMessage "Failure! The cones were too far apart from each other.")
                      (goto _label Break)))))
              (:Completed
                ;[1 1 1] Success message
                (CallFunction|SendMessage "Success! The cones were placed correctly!")))))))))

(fn ConstructionScript)