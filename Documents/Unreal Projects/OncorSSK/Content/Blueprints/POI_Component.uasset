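; POI component for Trigger actors that shows a point of interest on the player's minimap and as an overhead icon.
; UpdateIcon clears the old overhead icon, then, if the trigger is visible, matches the saved game state and is not completed, picks an icon by drop-down type.
; It then re-adds a static minimap POI and spawns an OverHead_Icon above the owner.
; CallingRemoveButKeep removes the owner's minimap entries without destroying the actor.
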(event Custom|UpdateIcon
  (bind _returnvalue (Components|GetOwner))
  (Utilities|IsValid (Variables|Default|GetBP)
    (:Is%20Valid
      (Actor|DestroyActor (Variables|Default|GetBP)))
    (:Is%20Not%20Valid
      _))
  (bind _astrigger (Utilities|Casting|CastToTrigger (Components|GetOwner)))
  (if (and (not (Variables|/Game/Blueprints/Trigger.Trigger_C|GetInvisiblePOI _astrigger)) (Utilities|Enum|Equal(Enum) (Variables|/Game/Blueprints/Trigger.Trigger_C|GetGamestate _astrigger) (.GS (Utilities|Struct|BreakSave_Struct (.SaveStruct (CallFunction|GetSave))))))
    (bind _astrigger_2 (Utilities|Casting|CastToTrigger (Components|GetOwner)))
    (if (not (or (Utilities|Array|ContainsItem (.Completed_Lvls (Utilities|Struct|BreakSave_Struct (.SaveStruct (CallFunction|GetSave)))) (Utilities|String|ToString(Name) (Variables|/Game/Blueprints/Trigger.Trigger_C|GetLevel _astrigger_2))) (Variables|/Game/Blueprints/Trigger.Trigger_C|GetComplete _astrigger_2)))
      ;[1 1 1] Set "Icon_Imag" base on Drop Down Sel
      (switch Utilities|FlowControl|Switch|SwitchonIcons (Variables|Default|GetDropDownSel)
        (:NewEnumerator1
          (Variables|Default|SetIcon_Imag "/Game/Textures/Danger_Icon.Danger_Icon"))
        (:NewEnumerator4
          (Variables|Default|SetIcon_Imag "/Game/Textures/Icon.Icon")))
      (bind _asthird_person_character (Utilities|Casting|CastToThirdPersonCharacter (Game|Player|GetPlayerPawn 0))
        (:then
          (Utilities|IsValid (Variables|Default|GetIconWidget)
            (:Is%20Valid
              (Widget|RemovefromParent (Variables|Default|GetIconWidget)))
            (:Is%20Not%20Valid
              _))
          (bind _newpoi (Default|AddPOI (Variables|/Game/Blueprints/SSK_HUD.SSK_HUD_C|GetMiniMap (Variables|/Game/ThirdPersonBP/Blueprints/ThirdPersonCharacter.ThirdPersonCharacter_C|GetHud _asthird_person_character)) true _returnvalue (Utilities|String|ToString(Name) (Variables|/Game/Blueprints/Trigger.Trigger_C|GetLevel _astrigger_2))))
          (Variables|Default|SetIconWidget _newpoi)
          ;[1 1 1] Spawn over head icon
          (Utilities|IsValid (Variables|Default|GetBP)
            (:Is%20Not%20Valid
              (bind _astrigger_3 (Utilities|Casting|CastToTrigger (Components|GetOwner)))
              (if (not (Variables|/Game/Blueprints/Trigger.Trigger_C|GetInvisiblePOI _astrigger_3))
                (bind _returnvalue_2 (Game|SpawnActorfromClass "/Game/Blueprints/OverHead_Icon.OverHead_Icon_C" (Math|Transform|MakeTransform (+ (Transformation|GetActorLocation _returnvalue) "0, 0,100.000000") "0, 0, 0" "1,1,1") "Undefined" 0 0))
                (Variables|Default|SetBP _returnvalue_2)))))
        (:CastFailed
          (Development|PrintString "Hello"))))))

(event EventBeginPlay)

(fn CallingRemoveButKeep
  (bind _self self)
  (bind _returnvalue (Components|GetOwner _self))
  (bind _asthird_person_character (Utilities|Casting|CastToThirdPersonCharacter (Game|GetPlayerCharacter 0)))
  (Utilities|IsValid (Variables|/Game/ThirdPersonBP/Blueprints/ThirdPersonCharacter.ThirdPersonCharacter_C|GetHud _asthird_person_character)
    (:Is%20Valid
      (for _array_element (Variables|/Game/Blueprints/MiniMap.MiniMap_C|GetPoI_BMArray (Variables|/Game/Blueprints/SSK_HUD.SSK_HUD_C|GetMiniMap (Variables|/Game/ThirdPersonBP/Blueprints/ThirdPersonCharacter.ThirdPersonCharacter_C|GetHud _asthird_person_character)))
        (Default|RemoveButKeepActor _array_element _returnvalue))
      (Default|UpdatePoIBMArr (Variables|/Game/Blueprints/SSK_HUD.SSK_HUD_C|GetMiniMap (Variables|/Game/ThirdPersonBP/Blueprints/ThirdPersonCharacter.ThirdPersonCharacter_C|GetHud _asthird_person_character)) _returnvalue))))