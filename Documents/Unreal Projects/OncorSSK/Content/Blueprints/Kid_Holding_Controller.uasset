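; Kid character Blueprint that poses a skeletal kid holding a game controller through its Oncor SSK animation Blueprint.
; Shortly after BeginPlay it turns the controller pose fully on and passes a talking flag to the AnimBP.
; Each tick, while a player pawn exists, it moves a look-at point onto an optional followed actor and feeds left and right thumb marker positions into the AnimBP.
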(event Collision|EventActorBeginOverlap
  (params (OtherActor :type Actor%20Object%20Reference)))

(event EventTick
  (params (DeltaSeconds :type Float%20%28single-precision%29))
  (bind _followingactor (Variables|Default|GetFollowingActor))
  (|CallParentFunction DeltaSeconds)
  (Utilities|IsValid (Game|Player|GetPlayerPawn 0)
    (:Is%20Valid
      (Utilities|FlowControl|Sequence
        (:then_0
          (Utilities|IsValid _followingactor
            (:Is%20Valid
              (Transformation|SetWorldLocation (Variables|Default|GetLookAtPoint) (Transformation|GetActorLocation _followingactor) false false))))
        (:then_1
          (bind _asoncor_ssk_skeleton_anim_blueprint (Utilities|Casting|CastToOncor_SSK_Skeleton_AnimBlueprint (Components|SkeletalMesh|GetAnimInstance (Variables|Default|GetSkeletalMesh))))
          (Variables|/Game/Models/Oncor_SSK_Skeleton_AnimBlueprint.Oncor_SSK_Skeleton_AnimBlueprint_C|SetLeftThumbPosition _asoncor_ssk_skeleton_anim_blueprint (Variables|/Script/Engine.SceneComponent|GetRelativeLocation (Variables|Default|GetLeftPosition)))
          (Variables|/Game/Models/Oncor_SSK_Skeleton_AnimBlueprint.Oncor_SSK_Skeleton_AnimBlueprint_C|SetRightThumbPosition _asoncor_ssk_skeleton_anim_blueprint (Variables|/Script/Engine.SceneComponent|GetRelativeLocation (Variables|Default|GetRightPosition))))))))

(event EventBeginPlay
  (|CallParentFunction)
  (Utilities|FlowControl|Delay 0.2)
  (bind _asoncor_ssk_skeleton_anim_blueprint (Utilities|Casting|CastToOncor_SSK_Skeleton_AnimBlueprint (Components|SkeletalMesh|GetAnimInstance (Variables|Default|GetSkeletalMesh))))
  (Variables|/Game/Models/Oncor_SSK_Skeleton_AnimBlueprint.Oncor_SSK_Skeleton_AnimBlueprint_C|SetControllerAlpha _asoncor_ssk_skeleton_anim_blueprint 1.0)
  (Variables|/Game/Models/Oncor_SSK_Skeleton_AnimBlueprint.Oncor_SSK_Skeleton_AnimBlueprint_C|SetTalking _asoncor_ssk_skeleton_anim_blueprint (Variables|Default|GetControllerTalking)))

(fn ConstructionScript)